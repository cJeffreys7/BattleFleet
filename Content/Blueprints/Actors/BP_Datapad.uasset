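; BP_Datapad is an interactable datapad actor that feeds dialogue messages to the game.
; Outline events toggle custom depth on its mesh for highlighting.
; Each interaction looks up a DT_Dialogue row named from DataDialogueName and the current index, then queues it through GM_GameModeCoreLogic.
; The index advances per message and resets to 1 at a path's end, saving that position for optional continuation.
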(event EventSetObjectOutline
  (Rendering|SetRenderCustomDepth (Variables|Default|GetSM_DataPad) true))

(event EventClearObjectOutline
  (Rendering|SetRenderCustomDepth (Variables|Default|GetSM_DataPad) false))

(event EventInteractwithObject
  (CallFunction|AddNextDialoguetoQueue false))

(fn ConstructionScript)

(fn AddNextDialoguetoQueue
  (params (continueAfterPreviousDialogue :type Boolean))
  (if continueAfterPreviousDialogue
    (Variables|Default|SetcurrentDialogueIndex (+ (Variables|Default|GetpreviousDialogueIndex) 1)))
  (bind _returnvalue (Utilities|GetDataTableRow "/Game/Blueprints/DataTables/DT_Dialogue.DT_Dialogue" (Utilities|String|StringToName (Utilities|String|Append (Utilities|String|Replace (Variables|Default|GetdataDialogueName) " ") "_" (Utilities|String|ToString(Integer) (Variables|Default|GetcurrentDialogueIndex)))))
    (:then
      (Default|AddMessagetoQueue (CallFunction|GetGameModeCoreLogic) _returnvalue true)
      (if (Utilities|Struct|BreakS_Message _returnvalue)
        (Variables|Default|SetpreviousDialogueIndex (Variables|Default|GetcurrentDialogueIndex))
        (CallFunction|SetNextDialogueIndex 1)
        (else
          (Math|Integer|IncrementInt (Variables|Default|GetcurrentDialogueIndex)))))
    (:RowNotFound
      (Development|PrintString (Utilities|String|Append "***CANNOT FIND ROW " (Utilities|String|Append (Utilities|String|Replace (Variables|Default|GetdataDialogueName) " ") "_" (Utilities|String|ToString(Integer) (Variables|Default|GetcurrentDialogueIndex))) " IN DT_DIALOGUE***") true true "(R=0.500000,G=0.000000,B=0.006500,A=1.000000)" 5.0))))

(fn SetNextDialogueIndex
  (params (nextDialogueIndex :type Integer))
  (Variables|Default|SetcurrentDialogueIndex nextDialogueIndex))

(fn GetGameModeCoreLogic
  (return (.AsGM%20Game%20Mode%20Core%20Logic (Utilities|Casting|CastToGM_GameModeCoreLogic (Game|GetGameMode)))))
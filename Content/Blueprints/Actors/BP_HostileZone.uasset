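; Hostile zone actor that flags a human overspace player inside its detection sphere, sized from ZoneRange, and sends an NPC to intercept them.
; Overlap toggles the player's hostile state, clearing it one second after exit.
; A looping timer checks for a detected player, then pauses itself and asks that player to spawn a random InterceptingNPCs entry; nothing here resumes it.
; Random ship selection logic is present but disconnected.
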(event OnComponentBeginOverlap(DetectionRange)
  (params (OverlappedComponent :type Primitive%20Component%20Object%20Reference) (OtherActor :type Actor%20Object%20Reference) (OtherComp :type Primitive%20Component%20Object%20Reference) (OtherBodyIndex :type Integer) (bFromSweep :type Boolean) (SweepResult :type Hit%20Result%20Structure%20%28by%20ref%29))
  (bind _asbp_overspace_player (Utilities|Casting|CastToBP_OverspacePlayer OtherActor))
  (if (Default|GetIsHumanPlayer _asbp_overspace_player)
    (bind _output_get (Variables|Default|SetdetectedPlayer _asbp_overspace_player))
    (Default|ToggleHostileZone _output_get true)))

(event OnComponentEndOverlap(DetectionRange)
  (params (OverlappedComponent :type Primitive%20Component%20Object%20Reference) (OtherActor :type Actor%20Object%20Reference) (OtherComp :type Primitive%20Component%20Object%20Reference) (OtherBodyIndex :type Integer))
  (if (== OtherActor (Variables|Default|GetdetectedPlayer))
    (Utilities|FlowControl|Delay 1.0)
    (Default|ToggleHostileZone (Variables|Default|GetdetectedPlayer) false)
    (Variables|Default|SetdetectedPlayer 0)))

(event EventBeginPlay
  (Utilities|Time|SetTimerbyFunctionName 0 "InterceptPlayerInRange" 8.0 true))

(fn ConstructionScript
  (Components|Sphere|SetSphereRadius (Variables|Default|GetDetectionRange) (/ (Variables|Default|GetzoneRange) 2.0) false))

(fn InterceptPlayerinRange
  (bind _interceptingnpcs (Variables|Default|GetinterceptingNPCs))
  (Utilities|IsValid (Variables|Default|GetdetectedPlayer)
    (:Is%20Valid
      (Class|KismetSystemLibrary|PauseTimer 0 "InterceptPlayerInRange")
      (if (> (Utilities|Array|Length (Variables|Default|GetinterceptingNPCs)) 0)
        (Default|SpawnInterceptingNPC (Variables|Default|GetdetectedPlayer) (Utilities|Array|Get(acopy) _interceptingnpcs (Math|Random|RandomIntegerinRange 0 (Utilities|Array|LastIndex _interceptingnpcs))) "NewEnumerator4")))))
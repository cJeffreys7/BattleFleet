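; Overspace map anomaly that, on BeginPlay, spawns a derelict ship, friendly trader or abandoned cargo container at its location based on AnomalyType.
; Derelicts get random DT_BaseShips stats and status effects; traders reuse BP_OverspacePlayer as AI-controlled NPCs registered with the game mode.
; Derelict and cargo types set a radar indicator and store AnomalyActor, which RemoveAnomaly destroys along with indicator and anomaly.
; Other indicator setups remain unwired.
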(event EventBeginPlay
  (bind _array (Utilities|Array|MakeArray "NewEnumerator0" "NewEnumerator1"))
  (switch Utilities|FlowControl|Switch|SwitchonE_AnomalyTypes (Variables|Default|GetanomalyType)
    (:NewEnumerator0)
    (:NewEnumerator1
      (Default|SetRadarIndicator (Variables|Default|GetBP_RadarIndicator) "/Game/ProIconPack/Textures/Base_Icons/Square/T_SquareMask_45_256x256.T_SquareMask_45_256x256" "(R=1.000000,G=0.938686,B=0.093059,A=1.000000)")
      (bind _returnvalue (Utilities|GetDataTableRow "/Game/Blueprints/DataTables/DT_BaseShips.DT_BaseShips" (Utilities|String|StringToName (Utilities|String|EnumtoString (Utilities|Enum|ByteToEnumE_ShipNames (Math|Conversions|ToByte(Integer) (Math|Random|RandomIntegerinRange 1 (- (|GetNumEnumEntries) 1)))))))
        (:then
          (bind _returnvalue_2 (Game|SpawnActorfromClass "/Game/Pawns/BP_OverspaceShip.BP_OverspaceShip_C" (Transformation|GetActorTransform) "Undefined" self _returnvalue false true 0))
          (Variables|Default|SetanomalyActor _returnvalue_2)
          (if (> (Utilities|Array|Length _array) 0)
            (for _array_element _array
              (Default|AddStatusEffect _returnvalue_2 _array_element)))
          (Default|UpdateShipComponents _returnvalue_2 true)
          (Default|SwitchCamera _returnvalue_2 5))))
    (:NewEnumerator2)
    (:NewEnumerator3)
    (:NewEnumerator4)
    (:NewEnumerator10
      (bind _returnvalue_3 (Game|SpawnActorfromClass "/Game/Pawns/BP_OverspacePlayer.BP_OverspacePlayer_C" (Transformation|GetActorTransform) "Undefined" self "/Game/ProIconPack/Textures/Base_Icons/Square/T_SquareMask_45_256x256.T_SquareMask_45_256x256" "(R=0.187821,G=0.752942,B=0.450786,A=1.000000)" true 0))
      (Pawn|SpawnDefaultController _returnvalue_3)
      (Default|SetPlayerName _returnvalue_3 (Utilities|Text|ToText(String) (Variables|Default|GetnpcName)))
      (Default|AddOverspaceNPC (.AsGM%20Overspace%20Mode (Utilities|Casting|CastToGM_OverspaceMode (Game|GetGameMode))) _returnvalue_3))
    (:NewEnumerator5)
    (:NewEnumerator6
      (Default|SetRadarIndicator (Variables|Default|GetBP_RadarIndicator) "/Game/ProIconPack/Textures/Base_Icons/Hexagon/64x64/T_Hexa_Base_64x64.T_Hexa_Base_64x64" "(R=0.187821,G=0.752942,B=0.450786,A=1.000000)")
      (bind _returnvalue_4 (Game|SpawnActorfromClass "/Game/Blueprints/Actors/BP_CargoContainer.BP_CargoContainer_C" (Transformation|GetActorTransform) "Undefined" self 0))
      (Variables|Default|SetanomalyActor _returnvalue_4))
    (:NewEnumerator7)
    (:NewEnumerator8)
    (:NewEnumerator9)
    (:NewEnumerator11)
    (:NewEnumerator12)))

(fn ConstructionScript)

(fn RemoveIndicator
  (Widget|RemovefromParent (Default|GetRadarIndicator (Variables|Default|GetBP_RadarIndicator))))

(fn RemoveAnomaly
  (Actor|DestroyActor (Variables|Default|GetanomalyActor))
  (CallFunction|RemoveIndicator)
  (Actor|DestroyActor))
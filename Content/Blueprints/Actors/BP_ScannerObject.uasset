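; Scanner preview actor that shows ships, planets and bases as holograms, captured by a scene capture limited to itself.
; Ships and planets get socket-placed stat widgets; planets missing from the codex table play a scan timeline and add a codex entry.
; Planet menu scans build POI billboards from data tables, and timelines move and zoom the spring arm between them.
; Each focused POI updates scanner info and queues player messages offering scan, codex, dock or dialogue.
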(event Custom|SetScannerCamMarker
  (params (markerIndex :type Integer))
  (bind (_markerlocation _markerrotation) (CallFunction|GetMarkerCamLocationandRotation markerIndex))
  (Variables|Default|SetnewMarkerLocation _markerlocation)
  (Variables|Default|SetnewMarkerRotation _markerrotation)
  (Default|HideMessage (Variables|Default|Getplayer) false true)
  (bind _lerpalpha (Timeline|MoveScannerCam PlayFromStart)
    (:Update
      (CallFunction|SetMarkerCamLocationandRotation (Math|Vector|Lerp(Vector) (Variables|Default|GetcurrentMarkerLocation) (Variables|Default|GetnewMarkerLocation) _lerpalpha) (Math|Rotator|Lerp(Rotator) (Variables|Default|GetcurrentMarkerRotation) (Variables|Default|GetnewMarkerRotation) _lerpalpha true)))
    (:Finished
      (Variables|Default|SetcurrentMarkerLocation (Variables|Default|GetnewMarkerLocation))
      (Variables|Default|SetcurrentMarkerRotation (Variables|Default|GetnewMarkerRotation))
      (CallFunction|SetPOIScannerInfo markerIndex))))

(event Custom|ScanPlanet
  (params (planetName :type String))
  (bind _returnvalue (Utilities|GetDataTableRow "/Game/Blueprints/DataTables/DT_Planets.DT_Planets" (Utilities|String|StringToName planetName))
    (:then
      (Default|SetUnscannedPlanetInfo (Variables|Default|GetscannerInfo) _returnvalue)
      (Default|AddCodexEntry (Variables|Default|Getplayer) (Utilities|String|StringToName planetName) (Utilities|Struct|MakeS_CodexEntry (Utilities|Struct|BreakS_Planet _returnvalue) "/Game/Models/SM_Sphere.SM_Sphere" "NewEnumerator2"))
      (bind (_direction _coloralpha _opacityalpha) (Timeline|ScanningPlanet PlayFromStart)
        (:Update
          (Rendering|Material|SetVectorParameterValue (Variables|Default|GetscannerHologramMI) "Color" (Math|Color|Lerp(LinearColor) "(R=1.000000,G=0.149960,B=0.149960,A=1.000000)" "(R=0.000000,G=0.300544,B=0.871367,A=0.000000)" _coloralpha) :!class /Script/Engine.MaterialInstanceDynamic)
          (Rendering|Material|SetScalarParameterValue (Variables|Default|GetscannerHologramMI) "Opacity" _opacityalpha :!class /Script/Engine.MaterialInstanceDynamic))
        (:Finished
          (CallFunction|SetPlanetMenuScan planetName))))
    (:RowNotFound
      (Development|PrintString (Utilities|String|Append "***UNABLE TO FIND ROW NAME " planetName " IN DT_PLANETS***") true true "(R=0.500000,G=0.000000,B=0.000000,A=1.000000)"))))

(event Custom|ToggleMarkerZoom
  (params (isZoomingIn :type Boolean))
  (if isZoomingIn
    (bind _lengthalpha (Timeline|ZoomToMarker Play)
      (:Update
        (Variables|/Script/Engine.SpringArmComponent|SetTargetArmLength (Variables|Default|GetSpringArm) (Math|Float|Lerp (Variables|Default|GetpoiMaxZoom) (Variables|Default|GetpoiMinZoom) _lengthalpha))))
    (else
      (Timeline|ZoomToMarker Reverse))))

(event EventBeginPlay
  (Utilities|Array|Add (Variables|/Script/Engine.SceneCaptureComponent|GetShowOnlyActors (Variables|Default|GetSceneCaptureComponent2D)) self)
  (Utilities|Array|Add (Variables|Default|GetscannerStatWigets) (Variables|Default|GetScannerStat1))
  (Utilities|Array|Add (Variables|Default|GetscannerStatWigets) (Variables|Default|GetScannerStat2))
  (Utilities|Array|Add (Variables|Default|GetscannerStatWigets) (Variables|Default|GetScannerStat3))
  (Utilities|Array|Add (Variables|Default|GetscannerStatWigets) (Variables|Default|GetScannerStat4)))

(fn ConstructionScript)

(fn GetSceneCaptureTexture
  (return (Variables|/Script/Engine.SceneCaptureComponent2D|GetTextureTarget (Variables|Default|GetSceneCaptureComponent2D))))

(fn SetSceneCaptureTexture
  (params (TextureTarget :type Texture%20Render%20Target%202D%20Object%20Reference))
  (Variables|/Script/Engine.SceneCaptureComponent2D|SetTextureTarget (Variables|Default|GetSceneCaptureComponent2D) TextureTarget))

(fn SetScannerObject
  (params (scannerObject :type Actor%20Object%20Reference))
  (CallFunction|ClearScannerStats)
  (bind _asbp_overspace_player (Utilities|Casting|CastToBP_OverspacePlayer scannerObject)
    (:then
      (Components|StaticMesh|SetStaticMesh (Variables|Default|GetScannerObject) (Default|GetShipMesh (Utilities|Array|Get(acopy) (Default|GetFleetShips _asbp_overspace_player))))
      (CallFunction|SetMeshScale 1.0)
      (CallFunction|SetMeshMaterials "/Game/Materials/Outline/MI_ScannerSchemaHologram.MI_ScannerSchemaHologram")
      (CallFunction|SetShipScannerStats (Default|GetAttacks (Utilities|Array|Get(acopy) (Default|GetFleetShips _asbp_overspace_player)))))
    (:CastFailed
      (bind _asbp_dockable_planet (Utilities|Casting|CastToBP_DockablePlanet scannerObject)
        (:then
          (Components|StaticMesh|SetStaticMesh (Variables|Default|GetScannerObject) (Default|GetBaseMesh _asbp_dockable_planet))
          (CallFunction|SetMeshScale 25.0)
          (CallFunction|SetMeshMaterials "/Game/Materials/Outline/MI_ScannerSchemaHologram.MI_ScannerSchemaHologram")
          (CallFunction|SetPlanetScannerStats (Utilities|Array|MakeArray "")))
        (:CastFailed
          (bind _asbp_dock_base (Utilities|Casting|CastToBP_DockBase scannerObject)
            (:then
              (Components|StaticMesh|SetStaticMesh (Variables|Default|GetScannerObject) (Default|GetBaseMesh _asbp_dock_base))
              (CallFunction|SetMeshScale 1.0)
              (CallFunction|SetMeshMaterials "/Game/Materials/Outline/MI_ScannerBaseHologram.MI_ScannerBaseHologram"))
            (:CastFailed
              (bind _asbp_overspace_ship (Utilities|Casting|CastToBP_OverspaceShip scannerObject)
                (:then
                  (Components|StaticMesh|SetStaticMesh (Variables|Default|GetScannerObject) (Default|GetShipMesh _asbp_overspace_ship))
                  (CallFunction|SetMeshScale 1.0)
                  (CallFunction|SetMeshMaterials "/Game/Materials/Outline/MI_ScannerSchemaHologram.MI_ScannerSchemaHologram")
                  (CallFunction|SetShipScannerStats (Default|GetAttacks _asbp_overspace_ship)))
                (:CastFailed
                  (Development|PrintString (Utilities|String|Append "***UNABLE TO SET SCANNER MESH FOR " (Utilities|GetDisplayName scannerObject) "***")))))))))))

(fn SetShipScannerStats
  (params (attacks :type Array%20of%20Texts))
  (for (_array_element _array_index) (Variables|Default|GetshipStatSockets)
    (if (Utilities|Array|IsValidIndex attacks _array_index)
      (Transformation|SetRelativeLocation (Utilities|Array|Get(acopy) (Variables|Default|GetscannerStatWigets) _array_index) (- (Transformation|GetSocketLocation (Variables|Default|GetScannerObject) _array_element) (Transformation|GetActorLocation)) false false)
      (Default|SetQuickStat (.AsW%20HUDScanner%20Stat (Utilities|Casting|CastToW_HUDScannerStat (UserInterface|GetUserWidgetObject (Utilities|Array|Get(acopy) (Variables|Default|GetscannerStatWigets) _array_index)))) (Utilities|String|ToString(Text) (Utilities|Array|Get(acopy) attacks _array_index)) (not (or (Utilities|Name|Equal(Name) _array_element "WeaponPoint1") (Utilities|Name|Equal(Name) _array_element "DockingPoint"))))
      (Default|ToggleScannerStat (.AsW%20HUDScanner%20Stat (Utilities|Casting|CastToW_HUDScannerStat (UserInterface|GetUserWidgetObject (Utilities|Array|Get(acopy) (Variables|Default|GetscannerStatWigets) _array_index)))) true))))

(fn SetMeshScale
  (params (scale :type Float%20%28single-precision%29))
  (Transformation|SetRelativeScale3D (Variables|Default|GetScannerObject) (Math|Vector|MakeVector scale scale scale)))

(fn SetMeshMaterials
  (params (meshMaterial :type Material%20Interface%20Object%20Reference))
  (for _array_element (Class|MeshComponent|GetMaterialSlotNames (Variables|Default|GetScannerObject))
    (Rendering|Material|SetMaterialbyName (Variables|Default|GetScannerObject) _array_element meshMaterial)))

(fn SetPlanetScannerStats
  (params (pointsOfInterest :type Array%20of%20Texts))
  (for (_array_element _array_index) (Variables|Default|GetplanetStatSockets)
    (if (Utilities|Array|IsValidIndex pointsOfInterest _array_index)
      (Transformation|SetRelativeLocation (Utilities|Array|Get(acopy) (Variables|Default|GetscannerStatWigets) _array_index) (- (Transformation|GetSocketLocation (Variables|Default|GetScannerObject) _array_element) (Transformation|GetActorLocation)) false false)
      (Default|SetQuickStat (.AsW%20HUDScanner%20Stat (Utilities|Casting|CastToW_HUDScannerStat (UserInterface|GetUserWidgetObject (Utilities|Array|Get(acopy) (Variables|Default|GetscannerStatWigets) _array_index)))) (Utilities|String|ToString(Text) (Utilities|Array|Get(acopy) pointsOfInterest _array_index)) (Math|Random|RandomBool))
      (Default|ToggleScannerStat (.AsW%20HUDScanner%20Stat (Utilities|Casting|CastToW_HUDScannerStat (UserInterface|GetUserWidgetObject (Utilities|Array|Get(acopy) (Variables|Default|GetscannerStatWigets) _array_index)))) true))))

(fn SetPlanetMenuScan
  (params (planetName :type String))
  (bind _returnvalue (Utilities|String|Replace planetName " "))
  (bind _returnvalue_2 (Utilities|String|StringToName _returnvalue))
  (Components|StaticMesh|SetStaticMesh (Variables|Default|GetScannerObject) "/Game/Models/SM_Sphere.SM_Sphere")
  (CallFunction|SetMeshScale 25.0)
  (Utilities|GetDataTableRow "/Game/Blueprints/DataTables/DT_CodexOfPlanets.DT_CodexOfPlanets" _returnvalue_2
    (:then
      (CallFunction|SetMeshMaterials "/Game/Materials/Outline/MI_ScannerSchemaHologram.MI_ScannerSchemaHologram")
      (bind _returnvalue_3 (Utilities|GetDataTableRow "/Game/Blueprints/DataTables/DT_Planets.DT_Planets" _returnvalue_2)
        (:then
          (bind _keys (Utilities|Map|Keys (Utilities|Struct|BreakS_Planet _returnvalue_3)))
          (Variables|Default|SetmarkerIndexes _keys)
          (bind _values (Utilities|Map|Values (Utilities|Struct|BreakS_Planet _returnvalue_3)))
          (Variables|Default|SetmarkerNames _values)
          (CallFunction|ClearScannerStats)
          (for (_array_element _array_index) (Variables|Default|GetmarkerNames)
            (bind _returnvalue_4 (Utilities|GetDataTableRow "/Game/Blueprints/DataTables/DT_POIs.DT_POIs" _array_element)
              (:then
                (Utilities|Array|Add (Variables|Default|GetplanetPOIs) _returnvalue_4)
                (bind _returnvalue_5 (AddComponent|AddMaterialBillboardComponent false (Math|Transform|MakeTransform (- (Transformation|GetSocketLocation (Variables|Default|GetScannerObject) (Utilities|Array|Get(acopy) (Variables|Default|GetplanetStatSockets) (Utilities|Array|Get(acopy) (Variables|Default|GetmarkerIndexes) _array_index))) (Transformation|GetActorLocation)))))
                (Utilities|Array|Add (Variables|Default|GetpoiMarkers) _returnvalue_5)
                (bind _returnvalue_6 (Rendering|Material|CreateDynamicMaterialInstance "/Game/Materials/HUD/M_Marker.M_Marker" "None" :!class /Script/Engine.KismetMaterialLibrary))
                (Rendering|Material|SetTextureParameterValue _returnvalue_6 "Texture" (.POITexture (Utilities|Struct|BreakS_PointOfInterest _returnvalue_4)))
                (Rendering|Material|SetVectorParameterValue _returnvalue_6 "Color" (Utilities|Select :Index (.POIType (Utilities|Struct|BreakS_PointOfInterest _returnvalue_4)) :NewEnumerator2 "" :NewEnumerator0 "(R=1.000000,G=0.149960,B=0.149960,A=1.000000)" :NewEnumerator1 "(R=0.187821,G=0.752942,B=0.450786,A=1.000000)") :!class /Script/Engine.MaterialInstanceDynamic)
                (Class|MaterialBillboardComponent|SetElements _returnvalue_5 (Utilities|Array|MakeArray (Utilities|Struct|MakeMaterialSpriteElement _returnvalue_6 0 false 128.0 128.0))))))
          (Variables|Default|SetcurrentMarkerLocation (Transformation|GetWorldLocation (Variables|Default|GetSpringArm)))
          (CallFunction|ViewNextScannerMarker false))
        (:RowNotFound
          (Development|PrintString (Utilities|String|Append "***UNABLE TO FIND ROW NAME " _returnvalue " IN DT_PLANETS***") true true "(R=0.500000,G=0.000000,B=0.000000,A=1.000000)"))))
    (:RowNotFound
      (bind _returnvalue_7 (Rendering|Material|CreateDynamicMaterialInstance "/Game/Materials/Outline/MI_ScannerSchemaHologram.MI_ScannerSchemaHologram" "None" :!class /Script/Engine.KismetMaterialLibrary))
      (bind _output_get (Variables|Default|SetscannerHologramMI _returnvalue_7))
      (CallFunction|SetMeshMaterials _output_get)
      (CallFunction|ScanPlanet _returnvalue))))

(fn GetMarkerCamLocationandRotation
  (params (markerIndex :type Integer))
  (bind _returnvalue (Transformation|GetActorLocation))
  (bind _scannerobject (Variables|Default|GetScannerObject))
  (bind _planetstatsockets (Variables|Default|GetplanetStatSockets))
  (bind _markerindexes (Variables|Default|GetmarkerIndexes))
  (bind _output (Utilities|Array|Get(acopy) _markerindexes markerIndex))
  (bind _output_2 (Utilities|Array|Get(acopy) _planetstatsockets _output))
  (bind _returnvalue_2 (Transformation|GetSocketLocation _scannerobject _output_2))
  (bind _returnvalue_3 (Math|Rotator|FindLookatRotation _returnvalue_2 _returnvalue))
  (bind (_roll _pitch _yaw) (Math|Rotator|BreakRotator _returnvalue_3))
  (return _returnvalue_2 (Math|Rotator|MakeRotator (Math|Float|MapRangeClamped _roll -1.8e+02 1.8e+02 -15.0 15.0) (Math|Float|MapRangeClamped _pitch -1.8e+02 1.8e+02 -15.0 15.0) _yaw)))

(fn SetMarkerCamLocationandRotation
  (params (newLocation :type Vector) (newRotation :type Rotator))
  (Transformation|SetWorldLocationAndRotation (Variables|Default|GetSpringArm) newLocation newRotation false false))

(fn SetScannerInfo
  (params (scannerInfo :type W%20Scanner%20Info%20Object%20Reference))
  (Variables|Default|SetscannerInfo scannerInfo))

(fn SetPOIScannerInfo
  (params (poiIndex :type Integer))
  (bind _planetpois (Variables|Default|GetplanetPOIs))
  (bind _output (Utilities|Array|Get(acopy) _planetpois poiIndex))
  (Default|SetPointOfInterestInfo (Variables|Default|GetscannerInfo) (select (Utilities|Struct|BreakS_PointOfInterest _output) "" _output))
  (CallFunction|SetScanAction _output poiIndex))

(fn ViewNextScannerMarker
  (params (viewNext :type Boolean))
  (if (!= (Math|Integer|Clamp(Integer) (+ (Variables|Default|GetmarkerIndex) (select viewNext 1 -1)) 0 (Utilities|Array|LastIndex (Variables|Default|GetmarkerNames))) (Variables|Default|GetmarkerIndex))
    (bind _output_get (Variables|Default|SetmarkerIndex (Math|Integer|Clamp(Integer) (+ (Variables|Default|GetmarkerIndex) (select viewNext 1 -1)) 0 (Utilities|Array|LastIndex (Variables|Default|GetmarkerNames)))))
    (CallFunction|SetScannerCamMarker _output_get)))

(fn SetScanAction
  (params (poi :type S%20Point%20Of%20Interest%20Structure) (poiIndex :type Integer))
  (bind (_poiname _description _startingdialogue) (Utilities|Struct|BreakS_PointOfInterest poi))
  (bind (_poitype _poiaction) (Utilities|Struct|BreakS_PointOfInterest poi))
  (bind _markerindex (Variables|Default|GetmarkerIndex))
  (bind _markernames (Variables|Default|GetmarkerNames))
  (bind _markerindex_2 (Variables|Default|GetmarkerIndex))
  (bind _returnvalue (Utilities|Array|LastIndex _markernames))
  (bind _returnvalue_2 (== _markerindex 0))
  (bind _returnvalue_3 (== _markerindex_2 _returnvalue))
  (LocalVariables|Setoption3 (select _returnvalue_2 "" "PREVIOUS AREA"))
  (LocalVariables|Setaction3 (select _returnvalue_2 "" "ViewNextScannerMarker_False"))
  (LocalVariables|Setoption4 (select _returnvalue_3 "" "NEXT AREA"))
  (LocalVariables|Setaction4 (select _returnvalue_3 "" "ViewNextScannerMarker_True"))
  (if (Utilities|Struct|BreakS_PointOfInterest poi)
    (Default|AddMessagetoQueue (Variables|Default|Getplayer) (Utilities|Struct|MakeS_Message "UNKOWN STRUCTURE DETECTED." "SCAN" "SCAN" (LocalVariables|Getoption2) (LocalVariables|Getaction2) (LocalVariables|Getoption3) (LocalVariables|Getaction3) (LocalVariables|Getoption4) (LocalVariables|Getaction4)) true)
    (else
      (switch Utilities|FlowControl|Switch|SwitchonE_ScanActions _poiaction
        (:NewEnumerator1
          (Default|AddMessagetoQueue (Variables|Default|Getplayer) (Utilities|Struct|MakeS_Message (Utilities|Text|FormatText "DEEP SCAN {POI Type}?" (Utilities|Text|ToText(String) (Utilities|String|EnumtoString _poitype))) "SCAN" "DeepScanPOI" (LocalVariables|Getoption2) (LocalVariables|Getaction2) (LocalVariables|Getoption3) (LocalVariables|Getaction3) (LocalVariables|Getoption4) (LocalVariables|Getaction4)) true))
        (:NewEnumerator2
          (Default|AddMessagetoQueue (Variables|Default|Getplayer) (Utilities|Struct|MakeS_Message (Utilities|Text|FormatText "ADD CODEX ENTRY FOR {POI Type}" (Utilities|Text|ToText(String) (Utilities|String|EnumtoString _poitype))) "ADD TO CODEX" (Utilities|Text|FormatText "AddToCodex_{EntryName}_{Description}_{StaticMesh}_{CodexTypeInt}" (Utilities|Text|ToText(String) (Utilities|String|ToString(Name) (Utilities|Array|Get(acopy) (Variables|Default|GetmarkerNames) poiIndex))) _description (Utilities|Text|MakeLiteralText "None") (Utilities|Text|MakeLiteralText "1")) (LocalVariables|Getoption2) (LocalVariables|Getaction2) (LocalVariables|Getoption3) (LocalVariables|Getaction3) (LocalVariables|Getoption4) (LocalVariables|Getaction4)) true))
        (:NewEnumerator3
          (Default|AddMessagetoQueue (Variables|Default|Getplayer) (Utilities|Struct|MakeS_Message (Utilities|Text|FormatText "DOCK AT {POI Type}?" _poiname) "DOCK" (Utilities|Text|FormatText "Dock_{levelName}_{baseName}" (Utilities|Text|FormatText "M_{baseName}" (Utilities|Text|ToText(String) (Utilities|String|Replace (Utilities|String|ToString(Text) _poiname) " "))) _poiname) (LocalVariables|Getoption2) (LocalVariables|Getaction2) (LocalVariables|Getoption3) (LocalVariables|Getaction3) (LocalVariables|Getoption4) (LocalVariables|Getaction4)) true))
        (:NewEnumerator4
          (bind _returnvalue_4 (Utilities|GetDataTableRow "/Game/Blueprints/DataTables/DT_Dialogue.DT_Dialogue" _startingdialogue)
            (:then
              (Default|AddMessagetoQueue (Variables|Default|Getplayer) _returnvalue_4 (Utilities|Struct|BreakS_Message _returnvalue_4)))
            (:RowNotFound
              (Development|PrintString (Utilities|String|Append "***UNABLE TO FIND ROW NAME " (Utilities|String|ToString(Name) _startingdialogue) " IN DT_DIALOGUE***") true true "(R=0.500000,G=0.000000,B=0.000000,A=1.000000)"))))))))

(fn SetPlayer
  (params (player :type BP%20Character%20Core%20Logic%20Object%20Reference))
  (Variables|Default|Setplayer player))

(fn DeepScanCurrentPOI
  (bind _currentpoi (CallFunction|GetScanCurrentPOI))
  (Default|SetPOIDeepScanInfo (Variables|Default|GetscannerInfo) _currentpoi)
  (bind _calculatedcombatlevel (CallFunction|CalculatePOICombatLevel _currentpoi))
  (return (Utilities|Struct|BreakS_PointOfInterest _currentpoi) _calculatedcombatlevel))

(fn CalculatePOICombatLevel
  (params (poi :type S%20Point%20Of%20Interest%20Structure))
  (bind _keys (Utilities|Map|Keys (Utilities|Struct|BreakS_PointOfInterest poi)))
  (for _array_element _keys
    (bind _returnvalue (Utilities|GetDataTableRow "/Game/Blueprints/DataTables/DT_MissionEvents.DT_MissionEvents" (Utilities|String|StringToName (Utilities|String|Replace (Utilities|String|EnumtoString _array_element) " ")))
      (:then
        (LocalVariables|SetcombatLevel (+ (.CombatLevel (Utilities|Struct|BreakS_MissionEvent _returnvalue)) (LocalVariables|GetcombatLevel))))))
  (return (LocalVariables|GetcombatLevel)))

(fn GetScanCurrentPOI
  (return (Utilities|Array|Get(acopy) (Variables|Default|GetplanetPOIs) (Variables|Default|GetmarkerIndex))))

(fn ScanCurrentPOI
  (CallFunction|SetPOIScannerInfo (Variables|Default|GetmarkerIndex)))

(fn ClearPlanetPOIMarkers
  (for _array_element (Variables|Default|GetpoiMarkers)
    (Components|DestroyComponent _array_element))
  (Utilities|Array|Clear (Variables|Default|GetpoiMarkers))
  (Variables|Default|SetmarkerIndex -1))

(fn ClearScannerStats
  (for _array_element (Variables|Default|GetscannerStatWigets)
    (Default|ToggleScannerStat (.AsW%20HUDScanner%20Stat (Utilities|Casting|CastToW_HUDScannerStat (UserInterface|GetUserWidgetObject _array_element))) false)))
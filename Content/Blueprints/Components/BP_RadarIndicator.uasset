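; BP_RadarIndicator is a component that registers its owning actor as an indicator on the player's radar.
; After short delays on BeginPlay, it gets the first player's radar from GM_OverspaceMode and passes it the owner, player and indicator appearance, offset and static settings.
; Human-controlled BP_CharacterCoreLogic owners are skipped, while AI characters and all other actors are registered.
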(event EventBeginPlay
  (Utilities|FlowControl|Delay 0.5)
  (bind _asbp_character_core_logic (Utilities|Casting|CastToBP_CharacterCoreLogic (Components|GetOwner))
    (:then
      (if (not (Default|GetIsHumanPlayer _asbp_character_core_logic))
        (Utilities|FlowControl|Delay 0.2 :!label _label)
        (bind _asgm_overspace_mode (Utilities|Casting|CastToGM_OverspaceMode (Game|GetGameMode)))
        (Default|AddRadarIndicator (Default|GetPlayerRadar _asgm_overspace_mode) (Components|GetOwner) (Default|GetPlayer _asgm_overspace_mode) (Variables|Default|GetindicatorTexture) (Variables|Default|GetindicatorColor) (Variables|Default|GetindicatorSize) (Variables|Default|GetisStatic) (Variables|Default|GetindicatorOffset))))
    (:CastFailed
      (goto _label))))
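; Roaming-mode character that registers with the game mode, swaps mesh and animation by gender, and handles interaction, officer data and weapon scrapping.
; For human players, Tick sphere-traces from the camera and outlines the interactable actor via custom depth on tagged components.
; Message events are underscore-delimited strings that FireEvent dispatches to dialogue, controller menus or level travel.
; Officer updates rebuild the DataTable through JSON, while scrapping saves schema ingredients to inventory through the game mode.
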(event Custom|SetMouseInput
  (params (isUI%20Input :type Boolean))
  (Default|SetMouseInput (CallFunction|GetCharacterController) isUI%20Input))

(event Custom|ExitDialogue
  (params (instant :type Boolean))
  (bind _playercontroller (CallFunction|GetCharacterController))
  (Variables|/Game/Controllers/BP_RoamingController.BP_RoamingController_C|SetinDialogue _playercontroller false)
  (Default|HideMessage (Default|GetCharacterHUD _playercontroller) false instant)
  (CallFunction|SetMouseInput false))

(event EventTick
  (params (DeltaSeconds :type Float%20%28single-precision%29))
  (bind _debugmessages (Variables|Default|GetdebugMessages))
  (bind _debugmessages_2 (Variables|Default|GetdebugMessages))
  ;[1 1 1] Highlight Interactable Actor
  (if (CallFunction|GetIsHumanPlayer)
    (bind (_hitresult _hitinteractable) (CallFunction|SphereTraceforInteractables 512.0 64.0))
    (if _hitinteractable
      (if (!= (.HitActor (Collision|BreakHitResult _hitresult)) (Variables|Default|GetinteractableActor))
        (CallFunction|SetActorOutline (.HitActor (Collision|BreakHitResult _hitresult)))
        (bind _output_get (Variables|Default|SetinteractableActor (.HitActor (Collision|BreakHitResult _hitresult))))
        (Development|PrintString (Utilities|String|Append "Set " (Utilities|String|ToString(Text) (Default|GetPlayerName (.AsBP%20Character (Utilities|Casting|CastToBP_Character _output_get)))) " as interactable actor") _debugmessages_2 _debugmessages_2 "(R=0.000000,G=1.000000,B=0.000000,A=1.000000)"))
      (elif (!= (Variables|Default|GetinteractableActor) 0)
        (Development|PrintString (Utilities|String|Append "Remove " (Utilities|String|ToString(Text) (Default|GetPlayerName (.AsBP%20Character (Utilities|Casting|CastToBP_Character (Variables|Default|GetinteractableActor))))) " as interactable actor") _debugmessages _debugmessages "(R=1.000000,G=1.000000,B=0.000000,A=1.000000)")
        (CallFunction|ClearActorOutline)
        (Variables|Default|SetinteractableActor 0)))))

(event EventBeginPlay
  (bind _asgm_roaming_character (Utilities|Casting|CastToGM_RoamingCharacter (Game|GetGameMode)))
  (bind _output_get (Variables|Default|SetroamingCharGM _asgm_roaming_character))
  (CallFunction|SetGameMode _output_get)
  (Utilities|FlowControl|Delay 0.5)
  (Variables|Default|SetenableBindings (CallFunction|GetIsHumanPlayer))
  (|CallParentFunction)
  (Default|RegisterPlayer (Variables|Default|GetroamingCharGM) self)
  (CallFunction|SetMessageOwner (Utilities|String|ToString(Text) (CallFunction|GetPlayerName))))

(event EventFireEventfromMessage
  (params (eventWithArguments :type String))
  (CallFunction|FireEvent eventWithArguments))

(event EventOnRegistration
  (params (success :type Boolean))
  (if success
    (bind _asbp_roaming_controller (Utilities|Casting|CastToBP_RoamingController (Pawn|GetController)))
    (bind _output_get (Variables|Default|SetroamingController _asbp_roaming_controller))
    (Default|SetPreviewPlayer _output_get (Default|GetAvatarbyName (CallFunction|GetGameMode) (CallFunction|GetPlayerName)))))

(event EventOnGenderChanged
  (params (NewGender :type Name :default "None"))
  ;[1 1 1] In addition to the default changes, also apply a new mesh and animation blueprint matching the mesh
  (|CallParentFunction NewGender)
  (bind _returnvalue (Utilities|GetDataTableRow "/Game/Action_Male_and_Female/Blueprints/Data/DT_Genders.DT_Genders" (CallFunction|GetActiveCustomizationbyKey "Gender"))
    (:then
      (Class|SkinnedMeshComponent|SetSkeletalMesh (Variables|Character|GetMesh) (.Mesh (Utilities|Struct|BreakFGenders _returnvalue)) false)
      (Components|SkeletalMesh|SetAnimInstanceClass (Variables|Character|GetMesh) (.AnimationBlueprint (Utilities|Struct|BreakFGenders _returnvalue))))))

(fn ConstructionScript
  (if (Variables|Default|GetupdateCharacter)
    (Variables|Default|SetupdateCharacter false)
    (|CallParentFunction)))

(fn SphereTraceforInteractables
  (params (range :type Float%20%28single-precision%29) (sphereRadius :type Float%20%28single-precision%29))
  (bind _followcamera (Variables|Default|GetFollowCamera))
  (bind _returnvalue (Transformation|GetWorldLocation _followcamera))
  (bind _returnvalue_2 (Math|Vector|GetForwardVector _followcamera))
  (bind _returnvalue_3 (* _returnvalue_2 range))
  (bind (_outhit _returnvalue_4) (Collision|SphereTraceByChannel (+ _returnvalue (/ _returnvalue_3 2.0)) (+ _returnvalue _returnvalue_3) sphereRadius "TraceTypeQuery3" false 0 "None"))
  (return _outhit _returnvalue_4))

(fn SetActorOutline
  (params (actor :type Actor%20Object%20Reference))
  (if (> (Utilities|Array|Length (Variables|Default|GetoutlineComponents)) 0)
    (CallFunction|ClearActorOutline))
  (for _array_element (Actor|GetComponentsbyTag actor "/Script/Engine.PrimitiveComponent" "Outline")
    (Utilities|Array|Add (Variables|Default|GetoutlineComponents) _array_element)
    (Rendering|SetRenderCustomDepth _array_element true))
  (return))

(fn ClearActorOutline
  (for _array_element (Variables|Default|GetoutlineComponents)
    (Rendering|SetRenderCustomDepth _array_element false))
  (Utilities|Array|Clear (Variables|Default|GetoutlineComponents))
  (return))

(fn GetInteractableActor
  (return (Variables|Default|GetinteractableActor)))

(fn FireEvent
  (params (eventWithArguments :type String))
  (bind _output_get (LocalVariables|SeteventArguments (Utilities|String|ParseIntoArray eventWithArguments "_")))
  (if (Utilities|Array|IsValidIndex _output_get)
    (switch string (Utilities|Array|Get(acopy) _output_get)
      (:Default
        (Development|PrintString (Utilities|String|Append "***UNABLE TO FIND ASSOCIATED EVENT FROM MESSAGE FOR " (Utilities|Array|Get(acopy) _output_get) "***") true true "(R=0.500000,G=0.000000,B=0.000000,A=1.000000)" 5.0))
      (:SetNextDialogue
        (|SetNextDialoguewithArguments))
      (:OpenTradeMenu
        (|OpenTradeMenuwithArguments))
      (:ExitDialogue
        (CallFunction|ExitDialogue false))
      (:ShowOfficerStats
        (|ShowOfficerStats))
      (:OpenFleetMenu
        (|OpenFleetMenuwithArguments))
      (:OpenCraftingMenu
        (|OpenCraftingMenu))
      (:LaunchFleet
        (|LaunchFleetwithArguments)))
    (else
      (Development|PrintString "***UNABLE TO SPLIT ARGUMENTS STRING FOR EVENT FROM MESSAGE***" true true "(R=0.500000,G=0.000000,B=0.000000,A=1.000000)" 5.0))))

(fn SetinInventory
  (params (inInventory :type Boolean))
  (Variables|Default|SetinInventory inInventory))

(fn GetInteractableCharacter
  (return (Variables|Default|GetinteractableCharacter)))

(fn SetInteractableCharacter
  (params (interactableCharacter :type BP%20Character%20Object%20Reference))
  (Variables|Default|SetinteractableCharacter interactableCharacter))

(fn SetOfficerData
  (params (updatedOfficer :type S%20Officer%20Structure))
  (bind _officersdatatable (LocalVariables|GetofficersDataTable))
  (LocalVariables|SetupdatedOfficerStats updatedOfficer)
  (bind _outrownames (DataTable|GetDataTableRowNames _officersdatatable))
  (LocalVariables|SetofficerIndex (Utilities|Array|FindItem _outrownames (Utilities|String|StringToName (Utilities|Struct|BreakS_Officer (LocalVariables|GetupdatedOfficerStats)))))
  (for (_array_element _array_index) _outrownames
    (bind _returnvalue (Utilities|GetDataTableRow _officersdatatable _array_element)
      (:then
        (bind _updatedofficerdata (Default|ParseOfficerDatatoJSON (CallFunction|GetGameMode) _array_index (select (>= (LocalVariables|GetofficerIndex) 0) (Utilities|Array|LastIndex _outrownames) (Utilities|Array|Length _outrownames)) _array_element (select (== (LocalVariables|GetofficerIndex) _array_index) (LocalVariables|GetupdatedOfficerStats) _returnvalue) (Variables|Default|GetofficerData)))
        (Variables|Default|SetofficerData _updatedofficerdata))))
  (if (>= (LocalVariables|GetofficerIndex) 0)
    _
    (else
      (if (Utilities|Enum|Equal(Enum) (Variables|Default|GetofficerData) "")
        (Variables|Default|SetofficerData "["))
      (bind _updatedofficerdata_2 (Default|ParseOfficerDatatoJSON (CallFunction|GetGameMode) (LocalVariables|GetofficerIndex) -1 (Utilities|String|StringToName (Utilities|Struct|BreakS_Officer (LocalVariables|GetupdatedOfficerStats))) (LocalVariables|GetupdatedOfficerStats) (Variables|Default|GetofficerData)))
      (Variables|Default|SetofficerData _updatedofficerdata_2)))
  (Default|UpdateDTfromJSON (CallFunction|GetGameMode) (Variables|Default|GetofficerData) _officersdatatable))

(fn SetOfficerAssignedShip
  (params (officer :type S%20Officer%20Structure%20%28by%20ref%29) (assignedShip :type String))
  (bind (_officername _officerthumbnail _aptitude _traits _assignedplayer _assignedship _officerhealth _officermaxhealth) (Utilities|Struct|BreakS_Officer officer))
  (return (Utilities|Struct|MakeS_Officer _officername _officerthumbnail _aptitude _traits _assignedplayer (Utilities|String|StringToName assignedShip) _officerhealth _officermaxhealth)))

(fn GetCharacterController
  (return (Variables|Default|GetroamingController)))

(fn ScrapWeapon
  (params (weaponName :type Text))
  (bind _returnvalue (Utilities|GetDataTableRow (Default|GetBaseInventoryDataTable (CallFunction|GetGameMode) "NewEnumerator2") (Utilities|String|StringToName (Utilities|String|Replace (Utilities|String|ToString(Text) weaponName) " ")))
    (:then
      (LocalVariables|Setschema _returnvalue)
      (bind _keys (Utilities|Map|Keys (Utilities|Struct|BreakS_BaseSchemaItem (LocalVariables|Getschema))))
      (for _array_element _keys
        (Utilities|Array|Add (LocalVariables|GetitemNames) (Utilities|String|EnumtoString _array_element)))
      (bind _values (Utilities|Map|Values (Utilities|Struct|BreakS_BaseSchemaItem (LocalVariables|Getschema))))
      (bind _success (CallFunction|AddNewInventoryItemsfromIngredients _values (LocalVariables|GetitemNames) "NewEnumerator0"))
      (if _success
        (Default|SaveInventory (CallFunction|GetGameMode) "NewEnumerator0" (Variables|Default|GetupdatedItems) (Utilities|String|ToString(Text) (CallFunction|GetPlayerName))))
      (Utilities|Array|Clear (LocalVariables|GetitemNames))
      (Utilities|Map|Clear (Variables|Default|GetupdatedItems))
      (bind _keys_2 (Utilities|Map|Keys (Utilities|Struct|BreakS_BaseSchemaItem (LocalVariables|Getschema))))
      (for _array_element_2 _keys_2
        (Utilities|Array|Add (LocalVariables|GetitemNames) (Utilities|String|EnumtoString _array_element_2)))
      (bind _values_2 (Utilities|Map|Values (Utilities|Struct|BreakS_BaseSchemaItem (LocalVariables|Getschema))))
      (bind _success_2 (CallFunction|AddNewInventoryItemsfromIngredients _values_2 (LocalVariables|GetitemNames) "NewEnumerator1"))
      (if _success_2
        (Default|SaveInventory (CallFunction|GetGameMode) "NewEnumerator1" (Variables|Default|GetupdatedItems) (Utilities|String|ToString(Text) (CallFunction|GetPlayerName))))
      (Utilities|Array|Clear (LocalVariables|GetitemNames))
      (Utilities|Map|Clear (Variables|Default|GetupdatedItems))
      (bind _keys_3 (Utilities|Map|Keys (Utilities|Struct|BreakS_BaseSchemaItem (LocalVariables|Getschema))))
      (for _array_element_3 _keys_3
        (Utilities|Array|Add (LocalVariables|GetitemNames) (Utilities|String|EnumtoString _array_element_3)))
      (bind _values_3 (Utilities|Map|Values (Utilities|Struct|BreakS_BaseSchemaItem (LocalVariables|Getschema))))
      (bind _success_3 (CallFunction|AddNewInventoryItemsfromIngredients _values_3 (LocalVariables|GetitemNames) "NewEnumerator2"))
      (if _success_3
        (Default|SaveInventory (CallFunction|GetGameMode) "NewEnumerator2" (Variables|Default|GetupdatedItems) (Utilities|String|ToString(Text) (CallFunction|GetPlayerName))))
      (Utilities|Array|Clear (LocalVariables|GetitemNames))
      (Utilities|Map|Clear (Variables|Default|GetupdatedItems))
      (bind _keys_4 (Utilities|Map|Keys (Utilities|Struct|BreakS_BaseSchemaItem (LocalVariables|Getschema))))
      (for _array_element_4 _keys_4
        (Utilities|Array|Add (LocalVariables|GetitemNames) (Utilities|String|EnumtoString _array_element_4)))
      (bind _values_4 (Utilities|Map|Values (Utilities|Struct|BreakS_BaseSchemaItem (LocalVariables|Getschema))))
      (bind _success_4 (CallFunction|AddNewInventoryItemsfromIngredients _values_4 (LocalVariables|GetitemNames) "NewEnumerator4"))
      (if _success_4
        (Default|SaveInventory (CallFunction|GetGameMode) "NewEnumerator4" (Variables|Default|GetupdatedItems) (Utilities|String|ToString(Text) (CallFunction|GetPlayerName)))))))

(fn EquipWeaponfromInventory
  (params (weaponName :type Text))
  (Utilities|Array|Add (LocalVariables|GetweaponComponents) (Utilities|String|Replace (Utilities|String|ToString(Text) weaponName) " "))
  (Utilities|Array|Add (LocalVariables|GetweaponAmounts) 1)
  (Default|RemoveInventoryItemsbyCategory (CallFunction|GetGameMode) (LocalVariables|GetweaponComponents) (LocalVariables|GetweaponAmounts) "NewEnumerator5" (Utilities|String|ToString(Text) (CallFunction|GetPlayerName))))

(fn AddNewInventoryItemsfromIngredients
  (params (itemAmounts :type Array%20of%20Integers) (itemNames :type Array%20of%20Strings) (itemCategory :type E_ItemTypes%20Enum :default "NewEnumerator0"))
  (for (_array_element _array_index) itemNames
    (if (.success (Default|GetBaseInventoryItemwithAmount (CallFunction|GetGameMode) itemCategory _array_element (Utilities|Array|Get(acopy) itemAmounts _array_index)))
      (Utilities|Map|Add (Variables|Default|GetupdatedItems) (LocalVariables|GetingredientName) (.inventoryItem (Default|GetBaseInventoryItemwithAmount (CallFunction|GetGameMode) itemCategory _array_element (Utilities|Array|Get(acopy) itemAmounts _array_index))))
      (else
        (Development|PrintString (Utilities|String|Append "***UNABLE TO FIND " _array_element " IN " (Utilities|String|EnumtoString itemCategory) "***") true true "(R=0.500000,G=0.000000,B=0.000000,A=1.000000)")
        (return false))))
  (return (> (Utilities|Map|Length (Variables|Default|GetupdatedItems)) 0)))
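; Shared character logic that holds name, human-player flag, game mode and HUD, and forwards UI, codex and message calls to them.
; Messages default their owner to the player and route to the battle, roaming or overspace game mode.
; Dialogue recursively queues DT_Dialogue rows keyed by name and index until an end-of-path flag.
; Helpers total per-level stat gains from curves (only Medium growth wired), space capitalized names and toggle mouse input.
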(fn ConstructionScript)

(fn AddMessagetoQueue
  (params (message :type S%20Message%20Structure%20%28by%20ref%29) (runMessageQueue :type Boolean))
  (bind (_message _option1 _action1 _option2 _action2 _option3 _action3 _option4 _action4 _autoprogresstime _eventtofire _eventtarget _messageowner _isdialogue _isenddialoguepath) (Utilities|Struct|BreakS_Message message))
  (CallFunction|SendMessagetoQueue (Variables|References|GetGameMode) (Utilities|Struct|MakeS_Message _message _option1 _action1 _option2 _action2 _option3 _action3 _option4 _action4 _autoprogresstime _eventtofire _eventtarget (select (== (Utilities|String|Len _messageowner) 0) (Variables|Dialogue|GetPlayerMessageOwner) _messageowner) _isdialogue _isenddialoguepath) runMessageQueue))

(fn SendMessagetoQueue
  (params (gameMode :type Game%20Mode%20Base%20Object%20Reference) (message :type S%20Message%20Structure) (runMessageQueue :type Boolean))
  (bind _asgm_battle_mode (Utilities|Casting|CastToGM_BattleMode gameMode)
    (:then
      (Default|AddMessagetoQueue _asgm_battle_mode message runMessageQueue))
    (:CastFailed
      (bind _asgm_roaming_character (Utilities|Casting|CastToGM_RoamingCharacter gameMode)
        (:then
          (Default|AddMessagetoQueue _asgm_roaming_character message runMessageQueue))
        (:CastFailed
          (bind _asgm_overspace_mode (Utilities|Casting|CastToGM_OverspaceMode gameMode))
          (Default|AddMessagetoQueue _asgm_overspace_mode message runMessageQueue))))))

(fn SetGameMode
  (params (GameMode :type GM%20Game%20Mode%20Core%20Logic%20Object%20Reference))
  (Variables|References|SetGameMode GameMode))

(fn SetIsHumanPlayer
  (params (IsHumanPlayer :type Boolean))
  (Variables|Player|SetIsHumanPlayer IsHumanPlayer))

(fn GetIsHumanPlayer
  (return (Variables|Player|GetIsHumanPlayer)))

(fn SetHUD
  (params (HUD :type W%20HUD%20Base%20Object%20Reference))
  (Variables|References|SetHUD HUD))

(fn GetHUD
  (return (Variables|References|GetHUD)))

(fn SetMessageOwner
  (params (PlayerMessageOwner :type String))
  (Variables|Dialogue|SetPlayerMessageOwner PlayerMessageOwner))

(fn GetPlayerName
  (return (Utilities|Text|ToText(String) (Variables|Player|GetPlayerName))))

(fn FireEventfromMessage
  (params (eventWithArguments :type String)))

(fn SetPlayerName
  (params (playerName :type Text))
  (Variables|Player|SetPlayerName (Utilities|String|ToString(Text) playerName)))

(fn GetGameMode
  (return (Variables|References|GetGameMode)))

(fn OnRegistration
  (params (success :type Boolean)))

(fn CalculateTotalStatsatLevel
  (params (proficiencyLevel :type Float%20%28single-precision%29) (growthSpeed :type E_GrowthSpeeds%20Enum :default "NewEnumerator0"))
  (bind _returnvalue (Math|Float|Truncate proficiencyLevel))
  (if (> _returnvalue 1)
    (for _index (range 2 _returnvalue)
      (LocalVariables|SetnewTotalHullGain (+ (LocalVariables|GetnewTotalHullGain) (Math|Curves|GetFloatValue (Utilities|Select :Index growthSpeed :NewEnumerator0 0 :NewEnumerator1 "/Game/Blueprints/Curves/MediumHullGain.MediumHullGain" :NewEnumerator2 0) (Math|Conversions|ToFloat(Integer) _index))))
      (LocalVariables|SetnewTotalShieldGain (+ (LocalVariables|GetnewTotalShieldGain) (Math|Curves|GetFloatValue (Utilities|Select :Index growthSpeed :NewEnumerator0 0 :NewEnumerator1 "/Game/Blueprints/Curves/MediumShieldGain.MediumShieldGain" :NewEnumerator2 0) (Math|Conversions|ToFloat(Integer) _index))))
      (LocalVariables|SetnewTotalSpeedGain (+ (LocalVariables|GetnewTotalSpeedGain) (Math|Curves|GetFloatValue (Utilities|Select :Index growthSpeed :NewEnumerator0 0 :NewEnumerator1 "/Game/Blueprints/Curves/MediumSpeedGain.MediumSpeedGain" :NewEnumerator2 0) (Math|Conversions|ToFloat(Integer) _index))))
      (LocalVariables|SetnewTotalAttackGain (+ (LocalVariables|GetnewTotalAttackGain) (Math|Curves|GetFloatValue (Utilities|Select :Index growthSpeed :NewEnumerator0 0 :NewEnumerator1 "/Game/Blueprints/Curves/MediumAttackGain.MediumAttackGain" :NewEnumerator2 0) (Math|Conversions|ToFloat(Integer) _index))))))
  (return (LocalVariables|GetnewTotalHullGain) (LocalVariables|GetnewTotalShieldGain) (LocalVariables|GetnewTotalSpeedGain) (LocalVariables|GetnewTotalAttackGain)))

(fn HideMessage
  (params (progressPostQueue :type Boolean) (instant :type Boolean))
  (Default|HideMessage (Variables|References|GetHUD) progressPostQueue instant))

(fn AddCodexEntry
  (params (entryName :type Name) (codexEntry :type S%20Codex%20Entry%20Structure) (staticMeshName :type String))
  (Default|AddCodexEntry (Variables|References|GetGameMode) entryName codexEntry staticMeshName))

(fn AddSpacestoCapitalizedName
  (params (spacelessName :type String))
  (bind _returnvalue (Utilities|String|MakeLiteralString spacelessName))
  (if (not (Utilities|String|Contains spacelessName " "))
    (for (_array_element _array_index) (Utilities|String|GetCharacterArrayfromString _returnvalue)
      (LocalVariables|SetnewName (Utilities|String|Append (LocalVariables|GetnewName) (select (and (and (>= (Utilities|String|GetCharacterasNumber _returnvalue _array_index) 65) (<= (Utilities|String|GetCharacterasNumber _returnvalue _array_index) 90)) (!= _array_index 0)) " " "") _array_element)))
    (return (LocalVariables|GetnewName))
    (else
      (Development|PrintString (Utilities|String|Append "\"" spacelessName "\" is already formatted with spaces") true true "(R=1.000000,G=0.500000,B=0.000000,A=1.000000)")
      (return spacelessName))))

(fn SetNextDialogueIndex
  (params (nextDialogueIndex :type Integer))
  (Variables|Dialogue|SetcurrentDialogueIndex nextDialogueIndex))

(fn PlayNextDialogue
  (params (updateAvatar :type Boolean) (character :type BP%20Character%20Base%20Object%20Reference) (characterNameOverride :type String))
  (bind _playername (CallFunction|GetPlayerName))
  (bind _returnvalue (Utilities|String|ToString(Text) _playername))
  (bind _returnvalue_2 (Utilities|Enum|Equal(Enum) characterNameOverride ""))
  (bind _returnvalue_3 (select _returnvalue_2 _returnvalue characterNameOverride))
  (if updateAvatar
    (Default|UpdateCharacterAvatar (Default|GetAvatarbyName (CallFunction|GetGameMode) _playername) (Utilities|String|StringToName _returnvalue_3) (Default|GetPlayerCurrentCustomizations character)))
  (CallFunction|AddNextDialoguetoQueue false _returnvalue_3))

(fn AddNextDialoguetoQueue
  (params (continueAfterPreviousDialogue :type Boolean) (characterNameOverride :type String))
  (bind _playername (CallFunction|GetPlayerName))
  (bind _returnvalue (Utilities|Enum|Equal(Enum) characterNameOverride ""))
  (bind _returnvalue_2 (Utilities|String|ToString(Text) _playername))
  (bind _returnvalue_3 (Utilities|String|SelectString _returnvalue_2 characterNameOverride _returnvalue))
  (bind _returnvalue_4 (Utilities|String|Replace _returnvalue_3 " "))
  (if continueAfterPreviousDialogue
    (Variables|Dialogue|SetcurrentDialogueIndex (+ (Variables|Dialogue|GetpreviousDialogueIndex) 1)))
  (LocalVariables|SetnewMessageOwner _returnvalue_4)
  (bind _returnvalue_5 (Utilities|GetDataTableRow "/Game/Blueprints/DataTables/DT_Dialogue.DT_Dialogue" (Utilities|String|StringToName (Utilities|String|Append _returnvalue_4 "_" (Utilities|String|ToString(Integer) (Variables|Dialogue|GetcurrentDialogueIndex)))))
    (:then
      (CallFunction|AddMessagetoQueue _returnvalue_5 true)
      (if (Utilities|Struct|BreakS_Message _returnvalue_5)
        (Variables|Dialogue|SetpreviousDialogueIndex (Variables|Dialogue|GetcurrentDialogueIndex))
        (CallFunction|SetNextDialogueIndex 1)
        (else
          (Math|Integer|IncrementInt (Variables|Dialogue|GetcurrentDialogueIndex)
            (:%20%20
              (CallFunction|AddNextDialoguetoQueue false (LocalVariables|GetnewMessageOwner)))))))
    (:RowNotFound
      (Development|PrintString (Utilities|String|Append "***CANNOT FIND ROW " (Utilities|String|Append _returnvalue_4 "_" (Utilities|String|ToString(Integer) (Variables|Dialogue|GetcurrentDialogueIndex))) " IN DT_DIALOGUE***") true true "(R=0.500000,G=0.000000,B=0.006500,A=1.000000)" 5.0))))

(fn ToggleMouseVisibility
  (params (setToVisible :type Boolean) (InWidgetToFocus :type Widget%20Object%20Reference) (playerController :type Player%20Controller%20Object%20Reference))
  (bind _debugmessages (Variables|Default|GetdebugMessages))
  (if setToVisible
    (Input|SetInputModeGameandUI playerController InWidgetToFocus "DoNotLock" true)
    (Variables|/Script/Engine.PlayerController|SetbShowMouseCursor playerController true)
    (else
      (Input|SetInputModeGameOnly playerController)
      (Variables|/Script/Engine.PlayerController|SetbShowMouseCursor playerController false)))
  (Development|PrintString (Utilities|String|Append "Set Mouse to " (Utilities|String|SelectString "Visible" "Hidden" (Variables|/Script/Engine.PlayerController|GetbShowMouseCursor playerController))) _debugmessages _debugmessages "(R=0.500000,G=0.000000,B=0.000000,A=1.000000)"))

(fn ShowOutcomeItems
  (params (outcomeItems :type Array%20of%20S%20Inventory%20Item%20Structures))
  (Default|ShowOutcomeItems (CallFunction|GetHUD) outcomeItems))
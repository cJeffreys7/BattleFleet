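; Officer character that rolls random stats, updates its avatar from current customizations and saves its profile.
; After BeginPlay delays, it picks a weighted aptitude and random trait into OfficerStats, which setters extend with player and ship assignments.
; Saving renders the game mode's avatar to a PNG icon and stores its filename as thumbnail.
; Name assignment rebuilds the gender-specific name DataTable as hand-built JSON to flag the name taken.
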(event Custom|SaveOfficerData
  (bind _gamemode (CallFunction|GetGameMode))
  (bind _playername (CallFunction|GetPlayerName))
  (bind _characteravatar (Default|GetAvatarbyName _gamemode _playername))
  (bind _returnvalue (Utilities|String|ToString(Text) _playername))
  (bind _scenecapture (Default|GetStillImageCaptureComponent _characteravatar))
  (bind _returnvalue_2 (Utilities|String|Append "T_" "CharacterIcon_" _returnvalue ".png"))
  (bind _returnvalue_3 (Rendering|CreateRenderTarget2D 256 256 "RTF_RGBA8"))
  (Variables|/Script/Engine.Texture|SetLODGroup _returnvalue_3 "TEXTUREGROUP_Character")
  (Variables|/Script/Engine.TextureRenderTarget|SetTargetGamma _returnvalue_3 1.15)
  (Default|SetIconPreviewTransform _characteravatar)
  (bind _output_get (Variables|/Script/Engine.SceneCaptureComponent2D|SetTextureTarget _scenecapture _returnvalue_3))
  (Rendering|SceneCapture|CaptureScene _scenecapture :!class /Script/Engine.SceneCaptureComponent2D)
  (Rendering|ExportRenderTarget _output_get (CallFunction|GetFilepath) _returnvalue_2)
  (bind _output_get_2 (Variables|Default|SetofficerStats (Utilities|Struct|MakeS_Officer (.OfficerName (Utilities|Struct|BreakS_Officer (Variables|Default|GetofficerStats))) _returnvalue_2 (.Aptitude (Utilities|Struct|BreakS_Officer (Variables|Default|GetofficerStats))) (.Traits (Utilities|Struct|BreakS_Officer (Variables|Default|GetofficerStats))) (.AssignedPlayer (Utilities|Struct|BreakS_Officer (Variables|Default|GetofficerStats))) (.AssignedShip (Utilities|Struct|BreakS_Officer (Variables|Default|GetofficerStats))))))
  (CallFunction|SetOfficerData _output_get_2))

(event EventBeginPlay
  (|CallParentFunction)
  (Utilities|FlowControl|Delay 1.0)
  (CallFunction|InitializeRandomOfficerStats)
  (Utilities|FlowControl|Delay 0.5)
  (Default|UpdateCharacterAvatar (Default|GetAvatarbyName (CallFunction|GetGameMode) (CallFunction|GetPlayerName)) "None" (CallFunction|GetPlayerCurrentCustomizations)))

(event Collision|EventActorBeginOverlap
  (params (OtherActor :type Actor%20Object%20Reference))
  (|CallParentFunction OtherActor))

(event EventTick
  (params (DeltaSeconds :type Float%20%28single-precision%29))
  (|CallParentFunction DeltaSeconds))

(event EventAddNextDialoguetoQueue
  (params (officer :type Boolean) (continueFromPrevious :type Boolean))
  (|CallParentFunction true false))

(fn ConstructionScript
  (|CallParentFunction))

(fn InitializeRandomOfficerStats
  (bind _output_get (LocalVariables|SetrandomPercentage (Math|Random|RandomIntegerinRange 0 99)))
  (if (<= _output_get 59)
    (LocalVariables|SetinitializedAptitude "NewEnumerator0")
    (elif (<= (LocalVariables|GetrandomPercentage) 89)
      (LocalVariables|SetinitializedAptitude "NewEnumerator1")
      (else
        (LocalVariables|SetinitializedAptitude "NewEnumerator2"))))
  (bind _outrownames (DataTable|GetDataTableRowNames "/Game/Blueprints/DataTables/DT_Traits.DT_Traits"))
  (Utilities|Array|Add (LocalVariables|GetinitializedTraits) (Utilities|Enum|ByteToEnumE_TraitTypes (Math|Conversions|ToByte(Integer) (Math|Random|RandomIntegerinRange 0 (Utilities|Array|LastIndex _outrownames)))))
  (Variables|Default|SetofficerStats (Utilities|Struct|MakeS_Officer (Utilities|String|ToString(Text) (CallFunction|GetPlayerName)) (LocalVariables|GetinitializedAptitude) (LocalVariables|GetinitializedTraits))))

(fn GetOfficerStats
  (return (Variables|Default|GetofficerStats)))

(fn GetTraits
  (return (.Traits (Utilities|Struct|BreakS_Officer (Variables|Default|GetofficerStats)))))

(fn AssignOfficerName
  (bind _output_get (LocalVariables|SetfemaleName (== (.Value (Utilities|Map|Find (Variables|Default|GetActiveCustomizationMap) "Gender")) 1)))
  (bind _outrownames (DataTable|GetDataTableRowNames (select _output_get "/Game/Blueprints/DataTables/DT_OfficerFemaleNames.DT_OfficerFemaleNames" "/Game/Blueprints/DataTables/DT_OfficerMaleNames.DT_OfficerMaleNames")))
  (for (_array_element _array_index) _outrownames
    (bind _returnvalue (Utilities|GetDataTableRow (select _output_get "/Game/Blueprints/DataTables/DT_OfficerFemaleNames.DT_OfficerFemaleNames" "/Game/Blueprints/DataTables/DT_OfficerMaleNames.DT_OfficerMaleNames") _array_element)
      (:then
        (if (Utilities|Enum|Equal(Enum) (.OfficerName (Utilities|Struct|BreakS_OfficerName _returnvalue)) (Utilities|Struct|BreakS_Officer (Variables|Default|GetofficerStats)))
          (if (.Assigned (Utilities|Struct|BreakS_OfficerName _returnvalue))
            (Development|PrintString (Utilities|String|Append "***NAME " (.OfficerName (Utilities|Struct|BreakS_OfficerName _returnvalue)) "IS ALREADY ASSIGNED IN " (Utilities|GetDisplayName (select _output_get "/Game/Blueprints/DataTables/DT_OfficerFemaleNames.DT_OfficerFemaleNames" "/Game/Blueprints/DataTables/DT_OfficerMaleNames.DT_OfficerMaleNames")) "***") true true "(R=0.500000,G=0.000000,B=0.010500,A=1.000000)"))
          (CallFunction|ParseOfficerNameDatatoJSON _array_index (Utilities|Array|Length _outrownames) (Utilities|Struct|MakeS_OfficerName (LocalVariables|GetfemaleName) (Utilities|Struct|BreakS_Officer (Variables|Default|GetofficerStats)) true))
          (LocalVariables|SetfoundName true)
          (else
            (CallFunction|ParseOfficerNameDatatoJSON _array_index (Utilities|Array|Length _outrownames) _returnvalue))))))
  (if (LocalVariables|GetfoundName)
    (CallFunction|UpdateDTfromJSON (Variables|Default|GetofficerNameData) (select _output_get "/Game/Blueprints/DataTables/DT_OfficerFemaleNames.DT_OfficerFemaleNames" "/Game/Blueprints/DataTables/DT_OfficerMaleNames.DT_OfficerMaleNames"))
    (else
      (Development|PrintString (Utilities|String|Append "***UNABLE TO FIND NAME " (.OfficerName (Utilities|Struct|BreakS_Officer (Variables|Default|GetofficerStats))) " IN " (Utilities|GetDisplayName (select _output_get "/Game/Blueprints/DataTables/DT_OfficerFemaleNames.DT_OfficerFemaleNames" "/Game/Blueprints/DataTables/DT_OfficerMaleNames.DT_OfficerMaleNames")) "***") true true "(R=0.500000,G=0.000000,B=0.010500,A=1.000000)"))))

(fn ParseOfficerNameDatatoJSON
  (params (nameIndex :type Integer) (totalNameCount :type Integer) (nameInfo :type S%20Officer%20Name%20Structure))
  (bind (_female _officername _assigned) (Utilities|Struct|BreakS_OfficerName nameInfo))
  (Variables|Default|SetofficerNameData (Utilities|String|Append (Utilities|String|SelectString "[" (Variables|Default|GetofficerNameData) (== nameIndex 0)) " 
   { 
" (Utilities|String|ToString(Text) (Utilities|Text|FormatText "      \"Name\": \"{RowName}\", 
      \"Female\": \"{Female}\", 
      \"OfficerName\": \"{OfficerName}\", 
      \"Assigned\": \"{Assigned}\"" (Utilities|Text|ToText(Integer) nameIndex false false) (Math|Conversions|ToByte(Integer) _female) (Utilities|Text|ToText(String) _officername) (Math|Conversions|ToByte(Integer) _assigned))) " 
   }" (Utilities|String|SelectString " 
]" "," (== nameIndex (- totalNameCount 1))))))

(fn SetAssignedPlayer
  (params (AssignedPlayer :type String))
  (Variables|Default|SetofficerStats (Utilities|Struct|MakeS_Officer (.OfficerName (Utilities|Struct|BreakS_Officer (Variables|Default|GetofficerStats))) "" (.Aptitude (Utilities|Struct|BreakS_Officer (Variables|Default|GetofficerStats))) (.Traits (Utilities|Struct|BreakS_Officer (Variables|Default|GetofficerStats))) AssignedPlayer (.AssignedShip (Utilities|Struct|BreakS_Officer (Variables|Default|GetofficerStats))))))

(fn SetAssignedShip
  (params (assignedShip :type String))
  (Variables|Default|SetofficerStats (Utilities|Struct|MakeS_Officer (.OfficerName (Utilities|Struct|BreakS_Officer (Variables|Default|GetofficerStats))) (.OfficerThumbnail (Utilities|Struct|BreakS_Officer (Variables|Default|GetofficerStats))) (.Aptitude (Utilities|Struct|BreakS_Officer (Variables|Default|GetofficerStats))) (.Traits (Utilities|Struct|BreakS_Officer (Variables|Default|GetofficerStats))) (.AssignedPlayer (Utilities|Struct|BreakS_Officer (Variables|Default|GetofficerStats))) (Utilities|String|StringToName assignedShip))))

(fn GetFilepath
  (return (Utilities|String|Append (Class|KismetSystemLibrary|GetProjectSavedDirectory) "AssetData\\AvatarIcons\\")))
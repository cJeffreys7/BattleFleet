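; BP_PlayerCoreLogic holds shared player logic, storing the game mode, HUD, human-player flag and default message owner behind simple accessors.
; AddMessageToQueue rebuilds each dialogue or message struct, substituting the player's owner name when none is supplied.
; FactorySendMessageToQueue then casts the stored game mode and forwards the message to GM_BattleMode, or otherwise GM_RoamingCharacter, so one call serves both modes.
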(event EventBeginPlay)

(event EventTick
  (params (DeltaSeconds :type Float%20%28single-precision%29)))

(fn AddMessagetoQueue
  (params (message :type S%20Message%20Structure%20%28by%20ref%29) (runMessageQueue :type Boolean))
  (bind (_message _option1 _action1 _option2 _action2 _option3 _action3 _option4 _action4 _autoprogresstime _eventtofire _eventtarget _messageowner _isdialogue _isenddialoguepath) (Utilities|Struct|BreakS_Message message))
  (CallFunction|FactorySendMessagetoQueue (Variables|Default|GetGameMode) (Utilities|Struct|MakeS_Message _message _option1 _action1 _option2 _action2 _option3 _action3 _option4 _action4 _autoprogresstime _eventtofire _eventtarget (select (== (Utilities|String|Len _messageowner) 0) (Variables|Default|GetPlayerMessageOwner) _messageowner) _isdialogue _isenddialoguepath) runMessageQueue))

(fn FactorySendMessagetoQueue
  (params (gameMode :type Game%20Mode%20Base%20Object%20Reference) (message :type S%20Message%20Structure) (runMessageQueue :type Boolean))
  (bind _asgm_battle_mode (Utilities|Casting|CastToGM_BattleMode gameMode)
    (:then
      (Default|AddMessagetoQueue _asgm_battle_mode message runMessageQueue))
    (:CastFailed
      (bind _asgm_roaming_character (Utilities|Casting|CastToGM_RoamingCharacter gameMode))
      (Default|AddMessagetoQueue _asgm_roaming_character message runMessageQueue))))

(fn SetMessageOwner
  (params (messageOwner :type String))
  (Variables|Default|SetPlayerMessageOwner messageOwner))

(fn SetGameMode
  (params (GameMode :type Game%20Mode%20Base%20Object%20Reference))
  (Variables|Default|SetGameMode GameMode))

(fn GetIsHuman
  (return (Variables|Default|GetIsHumanPlayer)))

(fn GetHUD
  (return (Variables|Default|GetHUD)))

(fn SetHUD
  (params (HUD :type W%20HUD%20Base%20Object%20Reference))
  (Variables|Default|SetHUD HUD))

(fn SetIsHuman
  (params (IsHumanPlayer :type Boolean))
  (Variables|Default|SetIsHumanPlayer IsHumanPlayer))
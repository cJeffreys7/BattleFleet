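; Force shield child actor that displays an expanding ring effect where a shield is hit.
; ShieldHit creates a dynamic hit material on its mesh and applies the supplied color and fade settings.
; The HitEffect timeline then drives ring radius and hardness, scaled by the hit parameters, positioning the hit as an offset from the mesh's world location.
; BeginPlay clears the lifespan, and nothing here destroys the actor.
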(event EventBeginPlay
  (Actor|SetLifeSpan -1.0))

(event EventShieldHit
  (params (HitLocation :type Vector :default "0, 0, 0") (Shield%20Scale :type Float%20%28single-precision%29) (Hit%20Ring%20Size%20Modifier :type Float%20%28single-precision%29) (Hit%20Ring%20Width%20Modifier :type Float%20%28single-precision%29) (Fade%20Distance :type Float%20%28single-precision%29) (Fade%20Opacity :type Float%20%28single-precision%29) (Color_01 :type Color%20Structure) (NewParam :type Boolean))
  (bind _returnvalue (Math|Conversions|ToLinearColor(Color) Color_01))
  (bind _mesh (Variables|Default|GetMesh))
  (bind _returnvalue_2 (Rendering|Material|CreateDynamicMaterialInstance _mesh 0 "/Game/ForceShields/Materials/Basic/M_ForceShield_HitBase.M_ForceShield_HitBase" "None" :!class /Script/Engine.PrimitiveComponent))
  (bind _output_get (Variables|Default|SetDynamic%20Material _returnvalue_2))
  (Rendering|Material|SetScalarParameterValue _output_get "Refraction" 1.0 :!class /Script/Engine.MaterialInstanceDynamic)
  (Rendering|Material|SetScalarParameterValue _output_get "Fade Distance" Fade%20Distance :!class /Script/Engine.MaterialInstanceDynamic)
  (Rendering|Material|SetScalarParameterValue _output_get "Fade Opacity" Fade%20Opacity :!class /Script/Engine.MaterialInstanceDynamic)
  (Rendering|Material|SetVectorParameterValue _output_get "Color_01" _returnvalue :!class /Script/Engine.MaterialInstanceDynamic)
  (Rendering|Material|SetVectorParameterValue _output_get "Color_02" _returnvalue :!class /Script/Engine.MaterialInstanceDynamic)
  (Rendering|Material|SetScalarParameterValue _output_get "Fresnel Expotent" 25.0 :!class /Script/Engine.MaterialInstanceDynamic)
  (bind _0_1 (Timeline|HitEffect PlayFromStart)
    (:Update
      (Rendering|Material|SetScalarParameterValue (Variables|Default|GetDynamic%20Material) "Radius" (* _0_1 (* Shield%20Scale Hit%20Ring%20Size%20Modifier)) :!class /Script/Engine.MaterialInstanceDynamic)
      (Rendering|Material|SetVectorParameterValue (Variables|Default|GetDynamic%20Material) "Hit Location" (Math|Conversions|ToLinearColor(Vector) (+ (Transformation|GetWorldLocation _mesh) HitLocation)) :!class /Script/Engine.MaterialInstanceDynamic)
      (Rendering|Material|SetScalarParameterValue (Variables|Default|GetDynamic%20Material) "Hardness" (* _0_1 Hit%20Ring%20Width%20Modifier) :!class /Script/Engine.MaterialInstanceDynamic))))

(fn ConstructionScript)
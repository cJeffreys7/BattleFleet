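; BP_Shields is a force shield actor that displays a configurable shield mesh with a shield material.
; The construction script runs the parent's, assigns ShieldMesh to the Mesh component, then applies ShieldMaterial to every material slot on it.
; The event graph holds only disabled placeholder events, so the Blueprint adds no runtime logic of its own.
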(event EventBeginPlay)

(event Collision|EventActorBeginOverlap
  (params (OtherActor :type Actor%20Object%20Reference)))

(event EventTick
  (params (DeltaSeconds :type Float%20%28single-precision%29)))

(fn ConstructionScript
  (|CallParentFunction)
  (Components|StaticMesh|SetStaticMesh (Variables|Character|GetMesh) (Variables|Default|GetshieldMesh))
  (for _index (range 0 (- (Rendering|Material|GetNumMaterials (Variables|Character|GetMesh)) 1))
    (Rendering|Material|SetMaterial (Variables|Character|GetMesh) _index (Variables|Default|GetShield%20Material))))
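; Game mode for turn-based ship battles that collects player confirmations, prompting NPCs to calculate actions until everyone has confirmed.
; Each ProgressBattleCycle call runs priority actions or, failing those, the fastest ship's action, starting the next cycle once none remain.
; It accumulates damage per attacker-target pair, and retrieving a ship's damage also purges records involving it.
; It also sets human players' cameras and plays a 2D sound on BeginPlay.
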(event Custom|CalculateFastestShip
  ;[0.5 0 0] Battle Cycle
  (Variables|ShipStats|SetfastestShipSpeed 0.0)
  (for _array_element (Variables|References|GetplayersConfirmedActions)
    (if (> (Utilities|Struct|BreakS_Ship (Default|GetShipStats (Variables|/Game/Pawns/BP_BattlePlayer.BP_BattlePlayer_C|GetActiveShip _array_element))) (Variables|ShipStats|GetfastestShipSpeed))
      (Variables|ShipStats|SetfastestShipSpeed (Utilities|Struct|BreakS_Ship (Default|GetShipStats (Variables|/Game/Pawns/BP_BattlePlayer.BP_BattlePlayer_C|GetActiveShip _array_element))))
      (Variables|ShipStats|SetfastestShip (Utilities|GetDisplayName (Variables|/Game/Pawns/BP_BattlePlayer.BP_BattlePlayer_C|GetActiveShip _array_element))))))

(event Custom|ProgressBattleCycle
  ;[0.5 0 0] Battle Cycle
  (if (> (Utilities|Array|Length (Variables|References|GetplayersConfirmedActions)) 0)
    (if (<= (Utilities|Array|Length (Variables|References|GetpriorityActions)) 0)
      (CallFunction|CalculateFastestShip)
      (|PerformActionbyFastestShip)
      (else
        (|PerformActionbyOrderofPriority)))
    (else
      (bind _result (Utilities|Set|ToArray (Variables|Default|Getplayers)))
      (for _array_element _result
        (bind _battleplayer (Utilities|CasttoBattlePlayer _array_element))
        (Default|StartNextBattleCycle _battleplayer)))))

(event Custom|PlayerActionConfirmed
  (params (player :type BP%20Battle%20Player%20Object%20Reference) (isPriority :type Boolean))
  (bind _debugmessages (Variables|Default|GetdebugMessages))
  ;[0.5 0 0] Battle Cycle
  (Development|PrintString (Utilities|String|Append (Utilities|String|ToString(Text) (Default|GetPlayerName player)) " confirmed Action") _debugmessages _debugmessages "(R=0.000000,G=0.820313,B=0.000000,A=1.000000)" 4.0)
  (Utilities|Array|AddUnique (Variables|References|GetplayersConfirmedActions) player)
  (if isPriority
    (Utilities|Array|AddUnique (Variables|References|GetpriorityActions) player))
  (if (== (Utilities|Array|Length (Variables|References|GetplayersConfirmedActions)) (Utilities|Set|Length (Variables|Default|Getplayers)))
    (CallFunction|ProgressBattleCycle)
    (else
      (for _array_element (Variables|Default|Getnpcs)
        (bind _battleplayer (Utilities|CasttoBattlePlayer _array_element))
        (Default|CalculateAIAction _battleplayer)))))

(event Custom|SetAllPlayersActiveCamera
  (params (cameraTarget :type Actor%20Object%20Reference) (cameraIndex :type Integer) (blendTime :type Float%20%28single-precision%29) (blendCurveExponent :type Float%20%28single-precision%29))
  ;[0 0.1845 0.4678] Camera Settings
  (bind _result (Utilities|Set|ToArray (Variables|Default|Getplayers)))
  (for _array_element _result
    (if (Default|GetIsHumanPlayer _array_element)
      (bind _battleplayer (Utilities|CasttoBattlePlayer _array_element))
      (Default|SetActiveCamera _battleplayer cameraTarget cameraIndex blendTime blendCurveExponent))))

(event EventBeginPlay
  ;[1 1 1] Set Sounds
  (|CallParentFunction)
  (Audio|PlaySound2D "/Game/SciFiGBigSoundPack/SoundPackCue/SciFiShipBackgroundSoundCue/InternalPremise4_Cue.InternalPremise4_Cue" 1.0 1.0 0.0 0 0))

(fn ConstructionScript)

(fn CheckifPlayerConfirmed
  (params (player :type BP%20Battle%20Player%20Object%20Reference%20%28by%20ref%29))
  (return (Utilities|Array|ContainsItem (Variables|References|GetplayersConfirmedActions) player)))

(fn RetrieveDamageAgainstShip
  (params (damagedShipName :type Text))
  (bind _returnvalue (Utilities|String|ToString(Text) damagedShipName))
  (bind _debugmessages (Variables|Default|GetdebugMessages))
  (for _array_element (Variables|Damage|GetdamageRecords)
    (Development|PrintString (Utilities|String|Append "Damage Record: " (.AttackingShipName (Utilities|Struct|BreakS_DamageRecord _array_element)) " inflicted " (Utilities|String|ToString(Float) (.Damage (Utilities|Struct|BreakS_DamageRecord _array_element))) " total damage on " (.DamagedShipName (Utilities|Struct|BreakS_DamageRecord _array_element))) _debugmessages _debugmessages "(R=0.000000,G=0.250000,B=0.000000,A=1.000000)")
    (if (Utilities|Enum|Equal(Enum) (.DamagedShipName (Utilities|Struct|BreakS_DamageRecord _array_element)) _returnvalue)
      (Utilities|Map|Add (LocalVariables|GetdamageResults) (.AttackingShipName (Utilities|Struct|BreakS_DamageRecord _array_element)) (.Damage (Utilities|Struct|BreakS_DamageRecord _array_element)))
      (Utilities|Array|Add (LocalVariables|GetretrievedDamageRecords) _array_element)
      (elif (Utilities|Enum|Equal(Enum) (.AttackingShipName (Utilities|Struct|BreakS_DamageRecord _array_element)) _returnvalue)
        (Utilities|Array|Add (LocalVariables|GetretrievedDamageRecords) _array_element))))
  (for _array_element_2 (LocalVariables|GetretrievedDamageRecords)
    (Utilities|Array|RemoveItem (Variables|Damage|GetdamageRecords) _array_element_2))
  (return (LocalVariables|GetdamageResults)))

(fn RecordDamageAgainstShip
  (params (attackingShipName :type Text) (damagedShipName :type Text) (damage :type Float%20%28single-precision%29))
  (bind _returnvalue (Utilities|String|ToString(Text) attackingShipName))
  (bind _returnvalue_2 (Utilities|String|ToString(Text) damagedShipName))
  (bind _debugmessages (Variables|Default|GetdebugMessages))
  (bind _debugmessages_2 (Variables|Default|GetdebugMessages))
  (if (Utilities|Array|IsValidIndex (Variables|Damage|GetdamageRecords))
    (for (_array_element _array_index) (Variables|Damage|GetdamageRecords)
      (if (and (Utilities|Enum|Equal(Enum) (.AttackingShipName (Utilities|Struct|BreakS_DamageRecord _array_element)) _returnvalue) (Utilities|Enum|Equal(Enum) (.DamagedShipName (Utilities|Struct|BreakS_DamageRecord _array_element)) _returnvalue_2))
        (Development|PrintString (Utilities|String|Append "Recorded " (Utilities|String|ToString(Float) damage) " damaged inflicted on " _returnvalue_2 " by " _returnvalue " (Total Damage = " (Utilities|String|ToString(Float) (+ (.Damage (Utilities|Struct|BreakS_DamageRecord _array_element)) damage)) ")") _debugmessages_2 _debugmessages_2)
        (Utilities|Array|SetArrayElem (Variables|Damage|GetdamageRecords) _array_index (Utilities|Struct|MakeS_DamageRecord (.AttackingShipName (Utilities|Struct|BreakS_DamageRecord _array_element)) (.DamagedShipName (Utilities|Struct|BreakS_DamageRecord _array_element)) (+ (.Damage (Utilities|Struct|BreakS_DamageRecord _array_element)) damage)))
        (return))))
  (Utilities|Array|Add (Variables|Damage|GetdamageRecords) (Utilities|Struct|MakeS_DamageRecord _returnvalue _returnvalue_2 damage))
  (Development|PrintString (Utilities|String|Append "Recorded " (Utilities|String|ToString(Float) damage) " damaged inflicted on " _returnvalue_2 " by " _returnvalue) _debugmessages _debugmessages)
  (return))
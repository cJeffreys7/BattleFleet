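; Core game mode logic that registers players and NPCs and runs a shared message and dialogue queue.
; Queued messages go to human players' HUDs, can fire named events on target players, and either auto-advance after a delay or enable HUD input.
; BeginPlay streams in a dialogue-image level of icon actors, which are assigned as avatars with render targets.
; Dialogue messages find their avatar texture by the owner's name prefix.
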(event Custom|RunMessageQueue
  (bind _messagequeue (Variables|Messages|GetmessageQueue))
  (bind _output (Utilities|Array|Get(acopy) _messagequeue))
  (bind (_autoprogresstime _eventtofire _eventtarget) (Utilities|Struct|BreakS_Message _output))
  ;[0.5906 0.8714 0.9387] Messages
  (Utilities|FlowControl|Delay (Variables|Messages|GetautoProgressMessageTime))
  (Variables|Messages|SetautoProgressMessageTime _autoprogresstime)
  (Variables|Messages|SeteventToFire _eventtofire)
  (Variables|Messages|SeteventTarget _eventtarget)
  (CallFunction|ProduceMessagetoHUDs)
  (CallFunction|FireMessageEvent)
  (if (or (== (Variables|Messages|GetautoProgressMessageTime) 0.0) (not (Utilities|Array|IsValidIndex (Variables|Messages|GetmessageQueue))))
    (CallFunction|EnableHUDInputs)
    (Variables|Messages|SetautoProgressMessageTime 0.0)
    (else
      (CallFunction|RunMessageQueue))))

(event Custom|RemoveMessagesByOwner
  (params (owner :type String))
  ;[0.5906 0.8714 0.9387] Messages
  (for _array_element (Variables|Messages|GetmessageQueue)
    (if (Utilities|Enum|Equal(Enum) (.MessageOwner (Utilities|Struct|BreakS_Message _array_element)) owner)
      (Utilities|Array|RemoveItem (Variables|Messages|GetmessageQueue) _array_element))))

(event Custom|ToggleLockScreens
  (params (lockScreens :type Boolean))
  ;[0.5906 0.8714 0.9387] Messages
  (bind _result (Utilities|Set|ToArray (Variables|References|Getplayers)))
  (bind _array_element (Utilities|Array|ForEachLoopwithBreak _result)
    (:LoopBody
      (if (Default|GetIsHumanPlayer _array_element)
        (Default|ToggleLockScreen (Default|GetHUD _array_element) lockScreens)))))

(event Custom|RegisterPlayer
  (params (player :type BP%20Character%20Core%20Logic%20Object%20Reference%20%28by%20ref%29))
  ;[0 0.1845 0.4678] References
  (Utilities|Set|Add (Variables|References|Getplayers) player)
  (if (Default|GetIsHumanPlayer player)
    (CallFunction|AssignPlayerAvatar player true)
    (else
      (Utilities|Array|AddUnique (Variables|References|Getnpcs) player)))
  (Default|OnRegistration player true))

(event Custom|AddMessageToQueue
  (params (message :type S%20Message%20Structure) (runMessageQueue :type Boolean))
  ;[0.5906 0.8714 0.9387] Messages
  (Utilities|Array|Add (Variables|Messages|GetmessageQueue) message)
  (if runMessageQueue
    (CallFunction|RunMessageQueue)))

(event Custom|FireMessageEvent
  ;[0.5906 0.8714 0.9387] Messages
  (if (> (Utilities|String|Len (Variables|Messages|GeteventToFire)) 0)
    (bind _result (Utilities|Set|ToArray (Variables|References|Getplayers)))
    (bind _array_element (Utilities|Array|ForEachLoopwithBreak _result)
      (:LoopBody
        (if (Utilities|Enum|Equal(Enum) (Utilities|String|ToString(Text) (Default|GetPlayerName _array_element)) (Variables|Messages|GeteventTarget))
          (Default|FireEventfromMessage _array_element (Variables|Messages|GeteventToFire)))))))

(event Custom|ProduceMessageToHUDs
  (bind _messagequeue (Variables|Messages|GetmessageQueue))
  (bind _output (Utilities|Array|Get(acopy) _messagequeue))
  (bind (_messageowner _isdialogue) (Utilities|Struct|BreakS_Message _output))
  ;[0.5906 0.8714 0.9387] Messages
  (bind _result (Utilities|Set|ToArray (Variables|References|Getplayers)))
  (for _array_element _result
    (if (Default|GetIsHumanPlayer _array_element)
      (if _isdialogue
        (Default|ConsumeNextMessage (Default|GetHUD _array_element) _output (Default|GetSceneCaptureTexture (CallFunction|GetAvatarbyName (Utilities|Text|ToText(String) (Utilities|Array|Get(acopy) (Utilities|String|ParseIntoArray _messageowner "_"))))))
        (else
          (Default|ConsumeNextMessage (Default|GetHUD _array_element) _output)))))
  (Utilities|Array|RemoveIndex (Variables|Messages|GetmessageQueue)))

(event Custom|EnableHUDInputs
  ;[0.5906 0.8714 0.9387] Messages
  (bind _result (Utilities|Set|ToArray (Variables|References|Getplayers)))
  (bind _array_element (Utilities|Array|ForEachLoopwithBreak _result)
    (:LoopBody
      (if (Default|GetIsHumanPlayer _array_element)
        (Default|EnableMessageInput (Default|GetHUD _array_element))))))

(event EventBeginPlay
  ;[0 0.1845 0.4678] References
  (Utilities|IsValid (Class|GameplayStatics|GetStreamingLevel "M_CharacterDialogueImage")
    (:Is%20Valid
      (Game|LoadStreamLevel(byName) "M_CharacterDialogueImage" true true)
      (bind _outactors (Actor|GetAllActorsOfClass "/Game/Action_Male_and_Female/Blueprints/Core/BP_Character_Dialogue_Icon.BP_Character_Dialogue_Icon_C"))
      (Variables|References|SetavailableCharacterAvatars _outactors))
    (:Is%20Not%20Valid
      (Development|PrintString "***M_CharacterDialogueImage MAP UNAVAILABLE TO STREAM***" (Variables|Default|GetdebugMessages) true "(R=0.500000,G=0.000000,B=0.001500,A=1.000000)" 5.0))))

(fn ConstructionScript)

(fn AssignAvailableAvatar
  (params (availableCharacterAvatars :type Array%20of%20BP%20Character%20Dialogue%20Icon%20Object%20References) (player :type BP%20Character%20Core%20Logic%20Object%20Reference))
  (bind _playername (Default|GetPlayerName player))
  (bind _output (Utilities|Array|Get(acopy) availableCharacterAvatars))
  (bind _assignedcharacteravatars (Variables|References|GetassignedCharacterAvatars))
  (bind _debugmessages (Variables|Default|GetdebugMessages))
  (bind _debugmessages_2 (Variables|Default|GetdebugMessages))
  (Development|PrintString (Utilities|String|Append (Utilities|String|ToString(Text) (Default|GetPlayerName player)) " is attempting to assign to available avatar") _debugmessages _debugmessages "(R=1.000000,G=1.000000,B=0.000000,A=1.000000)" 5.0)
  (bind _returnvalue (Utilities|Array|Add _assignedcharacteravatars _output))
  (Default|SetPlayerName (Utilities|Array|Get(acopy) _assignedcharacteravatars _returnvalue) _playername)
  (Development|PrintString (Utilities|String|Append "Assigned Avatar to " (Utilities|String|ToString(Text) _playername)) _debugmessages_2 _debugmessages_2 "(R=0.000000,G=1.000000,B=0.000000,A=1.000000)")
  (bind _returnvalue_2 (Rendering|CreateRenderTarget2D 256 256 "RTF_RGBA8"))
  (Default|SetSceneCaptureTexture (Utilities|Array|Get(acopy) _assignedcharacteravatars _returnvalue) _returnvalue_2)
  (return _output))

(fn GetAvatarbyName
  (params (playerName :type Text%20%28by%20ref%29))
  (for _array_element (Variables|References|GetassignedCharacterAvatars)
    (if (Utilities|Enum|Equal(Enum) (Default|GetPlayerName _array_element) playerName)
      (return _array_element)))
  (Development|PrintString (Utilities|String|Append "***NO CHARACTER AVATAR FOUND WITH NAME " (Utilities|String|ToString(Text) playerName) "***") (Variables|Default|GetdebugMessages) true "(R=0.500000,G=0.000000,B=0.000000,A=1.000000)" 5.0)
  (return 0))

(fn GetAnyMessages
  (return (Utilities|Array|IsValidIndex (Variables|Messages|GetmessageQueue))))

(fn AssignPlayerAvatar
  (params (player :type BP%20Character%20Core%20Logic%20Object%20Reference) (assignPermanently :type Boolean))
  (bind _availablecharacteravatars (Variables|References|GetavailableCharacterAvatars))
  (if (Utilities|Array|IsValidIndex _availablecharacteravatars)
    (bind _assignedplayer (CallFunction|AssignAvailableAvatar _availablecharacteravatars player))
    (if assignPermanently
      (Utilities|Array|RemoveItem (Variables|References|GetavailableCharacterAvatars) _assignedplayer))
    (else
      (Development|PrintString "***NO AVAILABLE CHARACTER AVATARS REMAINING***" (Variables|Default|GetdebugMessages) true "(R=0.500000,G=0.000000,B=0.000000,A=1.000000)" 5.0))))
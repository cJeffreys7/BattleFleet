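; Game mode for the Overspace map, restoring or spawning players and NPCs from a location DataTable and assigning a streamed scanner object to player one.
; A looping timer spawns anomalies ahead of that player up to a limit; NPC spawning and distance-culling logic exists but is unscheduled.
; It also runs missions, drawing random mandatory or chance-weighted events and queueing dialogue options from officer traits with pre-rolled success or failure outcomes.
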(event EventBeginPlay
  (|CallParentFunction)
  (Utilities|Time|SetTimerbyFunctionName 0 "CheckAnomaliesAroundPlayer" 1e+01 true)
  (Utilities|FlowControl|Delay 0.5)
  (bind _outactors (Actor|GetAllActorsOfClass "/Game/Pawns/BP_OverspacePlayer.BP_OverspacePlayer_C"))
  (for _array_element _outactors
    (if (Default|GetIsHumanPlayer _array_element)
      (Utilities|Array|Add (Variables|Default|GetoverspacePlayers) _array_element)
      (Utilities|Array|Add (Variables|Default|GetplayerNames) (Utilities|String|ToString(Text) (Default|GetPlayerName _array_element)))
      (else
        (Utilities|Array|Add (Variables|Default|GetoverspaceNPCs) _array_element)
        (Utilities|Array|Add (Variables|Default|GetnpcNames) (Utilities|String|ToString(Text) (Default|GetPlayerName _array_element))))))
  (bind _outrownames (DataTable|GetDataTableRowNames "/Game/Blueprints/DataTables/DT_OverspaceLocations.DT_OverspaceLocations"))
  (if (> (Utilities|Array|Length _outrownames) 0)
    (for _array_element_2 _outrownames
      (bind _returnvalue (Utilities|GetDataTableRow "/Game/Blueprints/DataTables/DT_OverspaceLocations.DT_OverspaceLocations" _array_element_2)
        (:then
          (if (>= (Utilities|Array|FindItem (Variables|Default|GetplayerNames) (.PlayerName (Utilities|Struct|BreakS_OverspaceLocation _returnvalue))) 0)
            (Transformation|SetActorLocation (Utilities|Array|Get(acopy) (Variables|Default|GetoverspacePlayers) (Utilities|Array|FindItem (Variables|Default|GetplayerNames) (.PlayerName (Utilities|Struct|BreakS_OverspaceLocation _returnvalue)))) (Math|Vector|MakeVector (.OverspaceLocationX (Utilities|Struct|BreakS_OverspaceLocation _returnvalue)) (.OverspaceLocationY (Utilities|Struct|BreakS_OverspaceLocation _returnvalue)) (.OverspaceLocationZ (Utilities|Struct|BreakS_OverspaceLocation _returnvalue))) false false)
            (elif (>= (Utilities|Array|FindItem (Variables|Default|GetnpcNames) (.PlayerName (Utilities|Struct|BreakS_OverspaceLocation _returnvalue))) 0)
              (Transformation|SetActorLocation (Utilities|Array|Get(acopy) (Variables|Default|GetoverspaceNPCs) (Utilities|Array|FindItem (Variables|Default|GetnpcNames) (.PlayerName (Utilities|Struct|BreakS_OverspaceLocation _returnvalue)))) (Math|Vector|MakeVector (.OverspaceLocationX (Utilities|Struct|BreakS_OverspaceLocation _returnvalue)) (.OverspaceLocationY (Utilities|Struct|BreakS_OverspaceLocation _returnvalue)) (.OverspaceLocationZ (Utilities|Struct|BreakS_OverspaceLocation _returnvalue))) false false)
              (else
                (bind _returnvalue_2 (Game|SpawnActorfromClass "/Game/Pawns/BP_OverspacePlayer.BP_OverspacePlayer_C" (Math|Transform|MakeTransform (Math|Vector|MakeVector (.OverspaceLocationX (Utilities|Struct|BreakS_OverspaceLocation _returnvalue)) (.OverspaceLocationY (Utilities|Struct|BreakS_OverspaceLocation _returnvalue)) (.OverspaceLocationZ (Utilities|Struct|BreakS_OverspaceLocation _returnvalue))) "0, 0, 0" "1,1,1") "Undefined" 0 "/Game/ProIconPack/Textures/Base_Icons/Square/T_SquareMask_45_256x256.T_SquareMask_45_256x256" "(R=1.000000,G=1.000000,B=1.000000,A=1.000000)" false 0))
                (if (Utilities|String|Contains (.PlayerName (Utilities|Struct|BreakS_OverspaceLocation _returnvalue)) "Player")
                  (Default|SetIsHumanPlayer _returnvalue_2 true)
                  (bind _returnvalue_3 (Game|SpawnActorfromClass (Variables|Default|GetPlayerControllerClass) (Transformation|GetActorTransform _returnvalue_2) "Undefined" 0 0))
                  (Pawn|Possess _returnvalue_3 _returnvalue_2)
                  (else
                    (Pawn|SpawnDefaultController _returnvalue_2)
                    (Utilities|Array|Add (Variables|Default|GetoverspaceNPCs) _returnvalue_2)))
                (Default|SetPlayerName _returnvalue_2 (Utilities|Text|ToText(String) (.PlayerName (Utilities|Struct|BreakS_OverspaceLocation _returnvalue)))))))))))
  (Utilities|IsValid (Class|GameplayStatics|GetStreamingLevel "M_Overspace_ScannedObject")
    (:Is%20Valid
      (Game|LoadStreamLevel(byName) "M_Overspace_ScannedObject" true true)
      (bind _outactors_2 (Actor|GetAllActorsOfClass "/Game/Pawns/BP_ScannerObject.BP_ScannerObject_C"))
      (Variables|Default|SetscannerObjects _outactors_2)
      (CallFunction|AssignScannerObjecttoPlayer))
    (:Is%20Not%20Valid
      (Development|PrintString "***M_Overspace_ScannedObject MAP UNAVAILABLE TO STREAM***" (Variables|Default|GetdebugMessages) true "(R=0.500000,G=0.000000,B=0.001500,A=1.000000)" 5.0))))

(fn ConstructionScript
  (|CallParentFunction))

(fn GetRandomForwardPeripheralLocation
  (params (player :type BP%20Overspace%20Player%20Object%20Reference))
  (bind _peripheralthreshold (Variables|Default|GetperipheralThreshold))
  (return (+ (Transformation|GetActorLocation player) (* (Math|Vector|GetForwardVector (Math|Rotator|CombineRotators (Default|GetFleetRotation player) (Math|Rotator|MakeRotator 0.0 0.0 (Math|Random|RandomFloatinRange (* (Variables|Default|GetforwardSightAngle) -1.0) (Variables|Default|GetforwardSightAngle))))) (Math|Random|RandomFloatinRange _peripheralthreshold (+ _peripheralthreshold (Variables|Default|GetperipheralRange)))))))

(fn SpawnAIPlayer
  (params (playerToSpawnNear :type BP%20Overspace%20Player%20Object%20Reference) (specifiedLocation :type Vector) (specifiedName :type String%20%28by%20ref%29))
  (bind _returnvalue (Game|SpawnActorfromClass "/Game/Pawns/BP_OverspacePlayer.BP_OverspacePlayer_C" (Math|Transform|MakeTransform (select (Math|Vector|NotEqual(Vector) specifiedLocation "0, 0, 0" 5.0) specifiedLocation (CallFunction|GetRandomForwardPeripheralLocation playerToSpawnNear)) "0, 0, 0" "1,1,1") "Undefined" 0 "/Game/ProIconPack/Textures/Base_Icons/Square/T_SquareMask_45_256x256.T_SquareMask_45_256x256" "(R=1.000000,G=1.000000,B=1.000000,A=1.000000)" false 0))
  (Pawn|SpawnDefaultController _returnvalue)
  (Default|SetPlayerName _returnvalue (Utilities|Text|ToText(String) (select (Utilities|Enum|NotEqual(Enum) specifiedName "") specifiedName (CallFunction|GetRandomAINameOfType "NPCRaider"))))
  (Utilities|Array|Add (Variables|Default|GetoverspaceNPCs) _returnvalue))

(fn GetRandomAINameOfType
  (params (npcType :type String))
  (bind _returnvalue (Math|Random|RandomIntegerinRange 1 2))
  (bind _returnvalue_2 (> _returnvalue 4))
  (Development|PrintString "Artemis has arrived!" _returnvalue_2 _returnvalue_2 "(R=1.000000,G=1.000000,B=0.000000,A=1.000000)")
  (return (select _returnvalue_2 "Artemis" (Utilities|String|Append npcType (Utilities|String|ToString(Integer) _returnvalue)))))

(fn RemoveOutOfRangeNPCs
  (params (player :type BP%20Overspace%20Player%20Object%20Reference))
  (bind _debugmessages (Variables|Default|GetdebugMessages))
  (for _array_element (Variables|Default|GetoverspaceNPCs)
    (if (>= (Transformation|GetHorizontalDistanceTo _array_element player) (Variables|Default|GetcullDistance))
      (Utilities|Array|Add (LocalVariables|GetnpcsToCull) _array_element)))
  (for _array_element_2 (LocalVariables|GetnpcsToCull)
    (Utilities|Array|RemoveItem (Variables|Default|GetoverspaceNPCs) _array_element_2)
    (Default|RemoveIndicator _array_element_2)
    (Actor|DestroyActor _array_element_2)
    (Development|PrintString "Removed out of range AI" _debugmessages _debugmessages "(R=1.000000,G=0.500000,B=0.000000,A=1.000000)"))
  (Utilities|Array|Clear (LocalVariables|GetnpcsToCull)))

(fn AddNPCstoPeripheralRange
  (params (playerToSpawnNear :type BP%20Overspace%20Player%20Object%20Reference))
  (bind _debugmessages (Variables|Default|GetdebugMessages))
  (if (< (Utilities|Array|Length (Variables|Default|GetoverspaceNPCs)) (Variables|Default|GetnpcCountLimit))
    (CallFunction|SpawnAIPlayer playerToSpawnNear "0, 0, 0" (Utilities|String|MakeLiteralString))
    (Development|PrintString (Utilities|String|Append "Spawning in AI - TOTAL: " (Utilities|String|ToString(Integer) (Utilities|Array|Length (Variables|Default|GetoverspaceNPCs)))) _debugmessages _debugmessages "(R=1.000000,G=1.000000,B=1.000000,A=1.000000)" 4.0)))

(fn CheckNPCsAroundPlayer
  (bind _overspaceplayers (Variables|Default|GetoverspacePlayers))
  (bind _output (Utilities|Array|Get(acopy) _overspaceplayers))
  (CallFunction|RemoveOutOfRangeNPCs _output)
  (CallFunction|RemoveOutOfRangeAnomalies _output)
  (CallFunction|AddNPCstoPeripheralRange _output))

(fn GetPlayerRadar
  (params (playerIndex :type Integer))
  (return (Default|GetRadar (.AsW%20Overspace%20HUD (Utilities|Casting|CastToW_OverspaceHUD (Default|GetHUD (CallFunction|GetPlayer playerIndex)))))))

(fn GetPlayer
  (params (playerIndex :type Integer))
  (return (Utilities|Array|Get(acopy) (Variables|Default|GetoverspacePlayers) playerIndex)))

(fn GetAvailableScannerObjects
  (return (Variables|Default|GetscannerObjects)))

(fn AssignScannerObjecttoPlayer
  (params (playerIndex :type Integer))
  (bind _scannerobjects (Variables|Default|GetscannerObjects))
  (bind _output (Utilities|Array|Get(acopy) _scannerobjects playerIndex))
  (if (Utilities|Array|IsValidIndex (Variables|Default|GetscannerObjects) playerIndex)
    (bind _returnvalue (Rendering|CreateRenderTarget2D 256 256 "RTF_RGBA8"))
    (Default|SetSceneCaptureTexture _output _returnvalue)
    (Default|SetScannerRenderObject (Utilities|Array|Get(acopy) (Variables|Default|GetoverspacePlayers) playerIndex) _output)
    (else
      (Development|PrintString (Utilities|String|Append "***NO VALID SCANNER OBJECT AT INDEX " (Utilities|String|ToString(Integer) playerIndex) "***") true true "(R=0.500000,G=0.000000,B=0.001500,A=1.000000)" 5.0))))

(fn LaunchMission
  (params (officers :type Array%20of%20S%20Officer%20Structures) (dropTrooperCount :type Integer) (missionPOI :type S%20Point%20Of%20Interest%20Structure) (missionPlayer :type BP%20Overspace%20Player%20Object%20Reference))
  (bind (_poiname _missionevents) (Utilities|Struct|BreakS_PointOfInterest missionPOI))
  (Variables|Missions|SetmissionPlayer missionPlayer)
  (Variables|Missions|SetmissionOfficers officers)
  (Variables|Missions|SetdropTrooperCount dropTrooperCount)
  (Variables|Missions|SetmissionPOIName (Utilities|String|ToString(Text) _poiname))
  (bind _keys (Utilities|Map|Keys _missionevents))
  (for _array_element _keys
    (bind _returnvalue (Utilities|GetDataTableRow "/Game/Blueprints/DataTables/DT_MissionEvents.DT_MissionEvents" (Utilities|String|StringToName (Utilities|String|Replace (Utilities|String|EnumtoString _array_element) " ")))
      (:then
        (Utilities|Array|Add (Variables|Missions|GetmissionEvents) _returnvalue)
        (if (Utilities|Struct|BreakS_MissionEvent _returnvalue)
          (Utilities|Array|Add (Variables|Missions|GetmandatoryEvents) _returnvalue)))
      (:RowNotFound
        (Development|PrintString (Utilities|String|Append "***UNABLE TO FIND ROW NAME " (Utilities|String|Replace (Utilities|String|EnumtoString _array_element) " ") " IN DT_MISSIONEVENTS***") true true "(R=0.500000,G=0.000000,B=0.000000,A=1.000000)"))))
  (CallFunction|SetNextMissionEvent))

(fn SetNextMissionEvent
  (bind _missionevents (Variables|Missions|GetmissionEvents))
  (bind _missionevent (CallFunction|GetRandomMission _missionevents))
  (bind (_chancetooccur _canrepeat) (Utilities|Struct|BreakS_MissionEvent _missionevent))
  (if (Math|Random|RandomBool)
    (if (CallFunction|GetAnyMandatoryEventsRemaining)
      (bind _output_get (Variables|Missions|SetcurrentEvent (CallFunction|GetRandomMission (Variables|Missions|GetmandatoryEvents)) :!label _label))
      (Utilities|Array|RemoveItem (Variables|Missions|GetmandatoryEvents) _output_get)
      (CallFunction|StartNextMissionEvent :!label _label_2)
      (elif (CallFunction|GetAnyMissionEventsRemaining)
        (if (> _chancetooccur (Math|Random|RandomFloatinRange 0.0 1e+02)) :!label _label_3
          (Variables|Missions|SetcurrentEvent _missionevent)
          (CallFunction|ReduceCurrentEventChance)
          (if _canrepeat
            (goto _label_2)
            (else
              (Utilities|Array|RemoveItem (Variables|Missions|GetmissionEvents) (Variables|Missions|GetcurrentEvent))
              (goto _label_2)))
          (else
            (Utilities|Array|RemoveItem (Variables|Missions|GetmissionEvents) _missionevent)
            (CallFunction|SetNextMissionEvent)))
        (else
          (CallFunction|EndMission :!label _label_4))))
    (elif (CallFunction|GetAnyMissionEventsRemaining)
      (goto _label_3)
      (elif (CallFunction|GetAnyMandatoryEventsRemaining)
        (goto _label)
        (else
          (goto _label_4))))))

(fn GetAnyMandatoryEventsRemaining
  (return (> (Utilities|Array|Length (Variables|Missions|GetmandatoryEvents)) 0)))

(fn GetAnyMissionEventsRemaining
  (return (> (Utilities|Array|Length (Variables|Missions|GetmissionEvents)) 0)))

(fn EndMission
  (Default|FinishMission (Variables|Missions|GetmissionPlayer)))

(fn GetRandomMission
  (params (missionEvents :type Array%20of%20S%20Mission%20Event%20Structures))
  (return (Utilities|Array|Get(acopy) missionEvents (Math|Random|RandomIntegerinRange 0 (Utilities|Array|LastIndex missionEvents)))))

(fn StartNextMissionEvent
  (bind _currentevent (Variables|Missions|GetcurrentEvent))
  (bind _eventoptions (LocalVariables|GeteventOptions))
  (bind _missionofficers (Variables|Missions|GetmissionOfficers))
  (bind (_description _chancetooccur _mustoccuratleastonce _canrepeat _combatlevel _successtraits _missionoptions _criticalsuccessdialogues _successdialogues _failuredialogues _criticalfailuredialogues) (Utilities|Struct|BreakS_MissionEvent _currentevent))
  (bind _textelement (CallFunction|GetTextArrayElement _eventoptions))
  (bind _returnvalue (Utilities|Text|TextIsEmpty _textelement))
  (bind _keys (Utilities|Map|Keys _missionoptions))
  (LocalVariables|SeteventTraitTypes _keys)
  (for _array_element (Variables|Missions|GetmissionOfficers)
    (for _array_element_2 (.Traits (Utilities|Struct|BreakS_Officer _array_element))
      (if (Utilities|Array|ContainsItem (LocalVariables|GeteventTraitTypes) _array_element_2)
        (CallFunction|SetMissionEventOptionandAction (LocalVariables|GeteventOptions) (LocalVariables|GeteventActions) (.OfficerName (Utilities|Struct|BreakS_Officer _array_element)) _array_element_2 _successtraits _missionoptions _criticalsuccessdialogues _successdialogues _failuredialogues _criticalfailuredialogues))))
  (if (< (Utilities|Array|Length (LocalVariables|GeteventOptions)) 3)
    (CallFunction|SetMissionEventOptionandAction (LocalVariables|GeteventOptions) (LocalVariables|GeteventActions) (.OfficerName (Utilities|Struct|BreakS_Officer (Utilities|Array|Get(acopy) _missionofficers (Math|Random|RandomIntegerinRange 0 (Utilities|Array|LastIndex _missionofficers))))) "NewEnumerator12" _successtraits _missionoptions _criticalsuccessdialogues _successdialogues _failuredialogues _criticalfailuredialogues))
  (CallFunction|AddMessagetoQueue (Utilities|Struct|MakeS_Message _description (select _returnvalue "Move On..." _textelement) (select _returnvalue "SetNextMissionEvent" (CallFunction|GetTextArrayElement (LocalVariables|GeteventActions))) (CallFunction|GetTextArrayElement (LocalVariables|GeteventOptions) 1) (CallFunction|GetTextArrayElement (LocalVariables|GeteventActions) 1) (CallFunction|GetTextArrayElement (LocalVariables|GeteventOptions) 2) (CallFunction|GetTextArrayElement (LocalVariables|GeteventActions) 2) (CallFunction|GetTextArrayElement (LocalVariables|GeteventOptions) 3) (CallFunction|GetTextArrayElement (LocalVariables|GeteventActions) 3) 0.0 "" "" (Utilities|String|ToString(Text) (Default|GetPlayerName (Variables|Missions|GetmissionPlayer)))) true))

(fn GetTextArrayElement
  (params (textArray :type Array%20of%20Texts) (index :type Integer))
  (if (Utilities|Array|IsValidIndex textArray index)
    (return (Utilities|Array|Get(acopy) textArray index))
    (else
      (return ""))))

(fn SetMissionEventOptionandAction
  (params (eventOptions :type Array%20of%20Texts) (eventActions :type Array%20of%20Texts) (officerName :type String) (officerTrait :type E_TraitTypes%20Enum :default "NewEnumerator0") (traitSuccessChances :type Map%20of%20E_TraitTypes%20Enums%20to%20Float%20%28single-precision%29s :default "NewEnumerator0") (traitOptions :type Map%20of%20E_TraitTypes%20Enums%20to%20Texts :default "NewEnumerator0") (traitCritSuccessAction :type Map%20of%20E_TraitTypes%20Enums%20to%20Texts :default "NewEnumerator0") (traitSuccessAction :type Map%20of%20E_TraitTypes%20Enums%20to%20Texts :default "NewEnumerator0") (traitFailureAction :type Map%20of%20E_TraitTypes%20Enums%20to%20Texts :default "NewEnumerator0") (traitCritFailureAction :type Map%20of%20E_TraitTypes%20Enums%20to%20Texts :default "NewEnumerator0"))
  (bind _debugmessages (Variables|Default|GetdebugMessages))
  (bind (_value _returnvalue) (Utilities|Map|Find traitSuccessAction officerTrait))
  (bind (_value_2 _returnvalue_2) (Utilities|Map|Find traitFailureAction officerTrait))
  (bind (_value_3 _returnvalue_3) (Utilities|Map|Find traitCritFailureAction officerTrait))
  (bind (_value_4 _returnvalue_4) (Utilities|Map|Find traitCritSuccessAction officerTrait))
  (bind _returnvalue_5 (Utilities|Array|AddUnique eventOptions (.Value (Utilities|Map|Find traitOptions officerTrait))))
  (if (> _returnvalue_5 -1)
    (if (<= _returnvalue_5 3)
      (LocalVariables|SetsuccessChance (.Value (Utilities|Map|Find traitSuccessChances officerTrait)))
      (if (> (LocalVariables|GetsuccessChance) (Math|Random|RandomFloatinRange 0.0 1e+02))
        (if (> 9.0 (Math|Random|RandomFloatinRange 0.0 1e+01))
          (LocalVariables|SetactionDialogue _value)
          (LocalVariables|SetdebugSuccessRating "SUCCESS")
          (LocalVariables|SetdebugFindAction _returnvalue)
          (else
            (LocalVariables|SetactionDialogue _value_4)
            (LocalVariables|SetdebugSuccessRating "CRITICAL SUCCESS")
            (LocalVariables|SetdebugFindAction _returnvalue_4)))
        (elif (> 9.0 (Math|Random|RandomFloatinRange 0.0 1e+01))
          (LocalVariables|SetactionDialogue _value_2)
          (LocalVariables|SetdebugSuccessRating "FAILURE")
          (LocalVariables|SetdebugFindAction _returnvalue_2)
          (else
            (LocalVariables|SetactionDialogue _value_3)
            (LocalVariables|SetdebugSuccessRating "CRITICAL FAILURE")
            (LocalVariables|SetdebugFindAction _returnvalue_3))))
      (Utilities|Array|Add eventActions (Utilities|Text|FormatText "StartSpecificDialogue_{RowName}_{OfficerName}_{OfficerTrait}" (LocalVariables|GetactionDialogue) (Utilities|Text|ToText(String) officerName) (Utilities|Text|ToText(String) (Utilities|String|Replace (Utilities|String|EnumtoString officerTrait) " "))))
      (if (LocalVariables|GetdebugFindAction)
        (Development|PrintString (Utilities|String|Append "SUCCESSFULLY ADDED EVENT ACTION: " (Utilities|String|ToString(Text) (Utilities|Text|FormatText "StartSpecificDialogue_{RowName}_{OfficerName}_{OfficerTrait}" (LocalVariables|GetactionDialogue) (Utilities|Text|ToText(String) officerName) (Utilities|Text|ToText(String) (Utilities|String|Replace (Utilities|String|EnumtoString officerTrait) " "))))) _debugmessages _debugmessages "(R=0.187821,G=0.752942,B=0.450786,A=1.000000)")
        (else
          (Development|PrintString (Utilities|String|Append "***UNABLE TO FIND OFFICER TRAIT " (Utilities|String|EnumtoString officerTrait) " IN " (LocalVariables|GetdebugSuccessRating) " DIALOGUES IN MISSION EVENT WITH DESCRIPTION: " (Utilities|String|ToString(Text) (Utilities|Struct|BreakS_MissionEvent (Variables|Missions|GetcurrentEvent))) "***") true true "(R=0.500000,G=0.000000,B=0.000000,A=1.000000)")))
      (else
        (Development|PrintString (Utilities|String|Append "***UNABLE TO PRESENT MORE THAN 4 OPTIONS IN DIALOGUE FOR MISSION. 
CONSIDER REFACTORING OR ALLOWING NO MORE THAN 4 MISSION EVENT OPTIONS FOR POI " (Variables|Missions|GetmissionPOIName) "***") true true "(R=0.500000,G=0.000000,B=0.000000,A=1.000000)")))))

(fn ReduceCurrentEventChance
  (bind _currentevent (Variables|Missions|GetcurrentEvent))
  (bind (_description _chancetooccur _mustoccuratleastonce _canrepeat _combatlevel _successtraits _missionoptions _criticalsuccessdialogues _successdialogues _failuredialogues _criticalfailuredialogues) (Utilities|Struct|BreakS_MissionEvent _currentevent))
  (Utilities|Array|SetArrayElem (Variables|Missions|GetmissionEvents) (Utilities|Array|FindItem (Variables|Missions|GetmissionEvents) (Variables|Missions|GetcurrentEvent)) (Utilities|Struct|MakeS_MissionEvent _description (Math|Float|Max(Float) (- _chancetooccur 1e+01) 0.0) _mustoccuratleastonce _canrepeat _combatlevel _successtraits _missionoptions _criticalsuccessdialogues _successdialogues _failuredialogues _criticalfailuredialogues)))

(fn CheckAnomaliesAroundPlayer
  (CallFunction|AddAnomalytoPeripheralRange (Utilities|Array|Get(acopy) (Variables|Default|GetoverspacePlayers))))

(fn RemoveOutOfRangeAnomalies
  (params (player :type BP%20Overspace%20Player%20Object%20Reference))
  (bind _debugmessages (Variables|Default|GetdebugMessages))
  (for _array_element (Variables|Default|Getanomalies)
    (if (>= (Transformation|GetHorizontalDistanceTo _array_element player) (Variables|Default|GetcullDistance))
      (Utilities|Array|Add (LocalVariables|GetanomaliesToCull) _array_element)))
  (for _array_element_2 (LocalVariables|GetanomaliesToCull)
    (Utilities|Array|RemoveItem (Variables|Default|Getanomalies) _array_element_2)
    (Default|RemoveAnomaly _array_element_2)
    (Development|PrintString "Removed out of range Anomaly" _debugmessages _debugmessages "(R=1.000000,G=0.500000,B=0.000000,A=1.000000)"))
  (Utilities|Array|Clear (LocalVariables|GetanomaliesToCull)))

(fn AddAnomalytoPeripheralRange
  (params (playerToSpawnNear :type BP%20Overspace%20Player%20Object%20Reference))
  (bind _debugmessages (Variables|Default|GetdebugMessages))
  (if (< (Utilities|Array|Length (Variables|Default|Getanomalies)) (Variables|Default|GetanomalyCountLimit))
    (CallFunction|SpawnAnomaly playerToSpawnNear "0, 0, 0" (Utilities|String|MakeLiteralString))
    (Development|PrintString (Utilities|String|Append "Spawning in Anomaly - TOTAL: " (Utilities|String|ToString(Integer) (Utilities|Array|Length (Variables|Default|Getanomalies)))) _debugmessages _debugmessages "(R=1.000000,G=1.000000,B=1.000000,A=1.000000)" 4.0)))

(fn SpawnAnomaly
  (params (playerToSpawnNear :type BP%20Overspace%20Player%20Object%20Reference) (specifiedLocation :type Vector) (specifiedName :type String%20%28by%20ref%29))
  (bind _returnvalue (Game|SpawnActorfromClass "/Game/Pawns/BP_OverspaceAnomaly.BP_OverspaceAnomaly_C" (Math|Transform|MakeTransform (select (Math|Vector|NotEqual(Vector) specifiedLocation "0, 0, 0" 5.0) specifiedLocation (CallFunction|GetRandomForwardPeripheralLocation playerToSpawnNear)) "0, 0, 0" "1,1,1") "Undefined" 0 "NewEnumerator1" (select (Utilities|Enum|NotEqual(Enum) specifiedName "") specifiedName "NPCTrader2") 0))
  (Utilities|Array|Add (Variables|Default|Getanomalies) _returnvalue))

(fn AddOverspaceNPC
  (params (newOverspaceNPC :type BP%20Overspace%20Player%20Object%20Reference%20%28by%20ref%29))
  (Utilities|Array|Add (Variables|Default|GetoverspaceNPCs) newOverspaceNPC))

(fn UnpauseTimers
  (Class|KismetSystemLibrary|UnPauseTimer 0 "CheckNPCsAroundPlayer")
  (Class|KismetSystemLibrary|UnPauseTimer 0 "CheckAnomaliesAroundPlayer"))

(fn PauseTimers
  (Class|KismetSystemLibrary|PauseTimer 0 "CheckNPCsAroundPlayer")
  (Class|KismetSystemLibrary|PauseTimer 0 "CheckAnomaliesAroundPlayer"))
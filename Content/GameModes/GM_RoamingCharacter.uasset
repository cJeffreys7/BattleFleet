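; GM_RoamingCharacter is a game mode that populates a hangar with the player's ships.
; It gathers target points tagged HangarDockPoint, then spawns a BP_ShipBase for each row of the DT_PlayerShips table at the dock point with the matching index, with idle movement off.
; Each ship receives its row's stats and status effects, updates its components, and is stored for lookup by index.
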(fn ConstructionScript)

(fn GetHangarDockingPoints
  (Utilities|Array|Clear (Variables|Default|GethangarDockingPoints))
  (bind _outactors (Actor|GetAllActorsOfClass "/Script/Engine.TargetPoint"))
  (for _array_element _outactors
    (if (Actor|ActorHasTag _array_element "HangarDockPoint")
      (Utilities|Array|Add (Variables|Default|GethangarDockingPoints) _array_element)))
  (return (Variables|Default|GethangarDockingPoints)))

(fn SpawnHangarShips
  (CallFunction|GetHangarDockingPoints)
  (bind _outrownames (DataTable|GetDataTableRowNames "/Game/Blueprints/DataTables/DT_PlayerShips.DT_PlayerShips"))
  (for (_array_element _array_index) _outrownames
    (bind _returnvalue (Utilities|GetDataTableRow "/Game/Blueprints/DataTables/DT_PlayerShips.DT_PlayerShips" _array_element)
      (:then
        (bind _returnvalue_2 (Game|SpawnActorfromClass "/Game/Pawns/BP_ShipBase.BP_ShipBase_C" (Math|Transform|MakeTransform (+ (.location (Transformation|GetActorTransform (Utilities|Array|Get(acopy) (Variables|Default|GethangarDockingPoints) _array_index))) "0, 0, 0") (.rotation (Transformation|GetActorTransform (Utilities|Array|Get(acopy) (Variables|Default|GethangarDockingPoints) _array_index))) (.scale (Transformation|GetActorTransform (Utilities|Array|Get(acopy) (Variables|Default|GethangarDockingPoints) _array_index)))) "Undefined" 0 _returnvalue false 0))
        (Utilities|Array|Add (Variables|Default|GethangarShips) _returnvalue_2)
        (if (> (Utilities|Array|Length (Utilities|Struct|BreakS_Ship _returnvalue)) 0)
          (for _array_element_2 (Utilities|Struct|BreakS_Ship _returnvalue)
            (Default|AddStatusEffect _returnvalue_2 _array_element_2)))
        (Default|UpdateShipComponents _returnvalue_2 true)))))

(fn GetHangarShipbyIndex
  (params (shipIndex :type Integer))
  (return (Utilities|Array|Get(acopy) (Variables|Default|GethangarShips) shipIndex)))
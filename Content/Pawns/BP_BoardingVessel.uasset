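; BP_BoardingVessel is a pawn asset that animates a boarding craft docking, presumably against a ship, with a success or failure outcome.
; Its BoardShip event snaps the DockingVessel component to a start offset, glides it inward, then runs two spark effects briefly.
; On failure, it spawns an explosion at the vessel, knocks it away with an eased tumble and hides the actor.
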(event Custom|BoardShip
  (params (success :type Boolean))
  (Components|MoveComponentTo (Variables|Default|GetDockingVessel) "500.000000, 0, 0" "0, 0, 0" false false 0.1 false)
  (Components|MoveComponentTo (Variables|Default|GetDockingVessel) "120.000000, 0, 0" "0, 0, 0" false false 2.0 false)
  (Components|Activation|Activate (Variables|Default|GetBoardingSparks1) false)
  (Components|Activation|Activate (Variables|Default|GetBoardingSparks2) false)
  (Utilities|FlowControl|Delay 2.0)
  (Components|Activation|Deactivate (Variables|Default|GetBoardingSparks1))
  (Components|Activation|Deactivate (Variables|Default|GetBoardingSparks2))
  (Utilities|FlowControl|Delay 1.0)
  (if (not success)
    (Effects|SpawnEmitteratLocation "/Game/Realistic_Starter_VFX_Pack_Vol2/Particles/Explosion/P_Explosion_Big_A.P_Explosion_Big_A" (Transformation|GetWorldLocation (Variables|Default|GetDockingVessel)))
    (Components|MoveComponentTo (Variables|Default|GetDockingVessel) "1000.000000, 0, 0" "0.000000,-45.000000,35.000000" true false 1.5 false)
    (Rendering|SetActorHiddenInGame true)))

(fn ConstructionScript)
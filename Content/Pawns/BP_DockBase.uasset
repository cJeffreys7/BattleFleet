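; BP_DockBase is a dockable base in overspace that offers docking to the human player on approach.
; Its construction script fills mesh, level, avatar and stats from the DT_Bases row named by BaseName, with UpdateBase forcing a refresh.
; Entering DetectionRange assigns the base's avatar and queues a Dock or Nevermind dialogue carrying a StopAllShips event.
; Entering ScanningRange makes the player scan the base.
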(event OnComponentBeginOverlap(DetectionRange)
  (params (OverlappedComponent :type Primitive%20Component%20Object%20Reference) (OtherActor :type Actor%20Object%20Reference) (OtherComp :type Primitive%20Component%20Object%20Reference) (OtherBodyIndex :type Integer) (bFromSweep :type Boolean) (SweepResult :type Hit%20Result%20Structure%20%28by%20ref%29))
  (bind _basename (Variables|Default|GetbaseName))
  (bind _returnvalue (Utilities|Text|ToText(String) _basename))
  (bind _asbp_overspace_player (Utilities|Casting|CastToBP_OverspacePlayer OtherActor))
  (if (Default|GetIsHumanPlayer _asbp_overspace_player)
    (bind _asgm_overspace_mode (Utilities|Casting|CastToGM_OverspaceMode (Game|GetGameMode)))
    (Default|QuickAssignPlayerAvatar _asgm_overspace_mode (Variables|Default|GetavatarName))
    (Default|AddMessagetoQueue _asbp_overspace_player (Utilities|Struct|MakeS_Message (Utilities|Text|FormatText "You are on an approach vector 
to {baseName}. 
State your business." _returnvalue) "Dock" (Utilities|Text|FormatText "Dock_{levelName}_{baseName}" (Variables|Default|GetbaseLevel) _returnvalue) "Nevermind" "ExitDialogue" "" "" "" "" 0.0 "StopAllShips" (Utilities|String|ToString(Text) (Default|GetPlayerName _asbp_overspace_player)) (Utilities|String|ToString(Text) (Variables|Default|GetavatarName)) true true) true)))

(event OnComponentBeginOverlap(ScanningRange)
  (params (OverlappedComponent :type Primitive%20Component%20Object%20Reference) (OtherActor :type Actor%20Object%20Reference) (OtherComp :type Primitive%20Component%20Object%20Reference) (OtherBodyIndex :type Integer) (bFromSweep :type Boolean) (SweepResult :type Hit%20Result%20Structure%20%28by%20ref%29))
  (bind _asbp_overspace_player (Utilities|Casting|CastToBP_OverspacePlayer OtherActor))
  (if (Default|GetIsHumanPlayer _asbp_overspace_player)
    (Default|ScanObject _asbp_overspace_player self)))

(fn ConstructionScript
  (bind _basename (Variables|Default|GetbaseName))
  (bind _returnvalue (Utilities|String|Replace _basename " "))
  (if (or (== (Variables|/Script/Engine.StaticMeshComponent|GetStaticMesh (Variables|Default|GetBaseMesh)) 0) (Variables|Default|GetupdateBase))
    (Variables|Default|SetupdateBase false)
    (bind _returnvalue_2 (Utilities|GetDataTableRow "/Game/Blueprints/DataTables/DT_Bases.DT_Bases" (Utilities|String|StringToName _returnvalue))
      (:then
        (bind _output_get (Variables|Default|SetbaseStats _returnvalue_2))
        (Components|StaticMesh|SetStaticMesh (Variables|Default|GetBaseMesh) (.BaseMesh (Utilities|Struct|BreakS_Base _output_get)))
        (Variables|Default|SetbaseLevel (Utilities|Text|ToText(String) (.BaseLevel (Utilities|Struct|BreakS_Base _output_get))))
        (Variables|Default|SetavatarName (.BaseAvatar (Utilities|Struct|BreakS_Base _output_get))))
      (:RowNotFound
        (Development|PrintString (Utilities|String|Append "***UNABLE TO FIND ROW NAME " _returnvalue " IN DT_BASES***") true true "(R=0.500000,G=0.000000,B=0.000000,A=1.000000)")))))

(fn GetBaseMesh
  (return (Variables|/Script/Engine.StaticMeshComponent|GetStaticMesh (Variables|Default|GetBaseMesh))))

(fn GetBaseStats
  (return (Variables|Default|GetbaseStats)))
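; Overspace fleet pawn for human and NPC players, carrying ships spawned from data tables into attached formation slots.
; Humans get a HUD plus speed-driven camera zoom, pitch and flight lag; NPCs run a behavior tree and steer toward a target or location.
; Engaging a target halts all fleets and queues dialogue.
; Underscore-delimited message strings trigger events such as battle or docking level loads, passing names as level options.
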(event Custom|SetMouseInput
  (params (isUI%20Input :type Boolean))
  (bind _returnvalue (Game|GetPlayerController 0))
  (Variables|/Script/Engine.PlayerController|SetbShowMouseCursor _returnvalue isUI%20Input)
  (if isUI%20Input
    (Input|SetInputModeGameandUI _returnvalue (Variables|Default|GetHUD) "DoNotLock" false)
    (else
      (Input|SetInputModeGameOnly _returnvalue))))

(event Custom|ExitDialogue
  (params (instant :type Boolean))
  (Default|HideMessage (CallFunction|GetHUD) false instant)
  (CallFunction|SetMouseInput false)
  (Utilities|FlowControl|Delay 1.0)
  (CallFunction|EnableAllShipsMovement))

(event EventBeginPlay
  (|CallParentFunction)
  (Utilities|FlowControl|Delay 0.5)
  (CallFunction|SpawnPlayerShips)
  (bind _asgm_overspace_mode (Utilities|Casting|CastToGM_OverspaceMode (Game|GetGameMode)))
  (CallFunction|SetGameMode _asgm_overspace_mode)
  (if (CallFunction|GetIsHumanPlayer)
    (Collision|SetCollisionProfileName (Variables|Default|GetPlayerCollision) "OverspacePlayerTrace" :!class /Script/Engine.PrimitiveComponent)
    (CallFunction|SetPlayerName "Player 1")
    (Default|RegisterPlayer (CallFunction|GetGameMode) self)
    (bind _asbp_overspace_controller (Utilities|Casting|CastToBP_OverspaceController (Pawn|GetController)))
    (bind _returnvalue (UserInterface|CreateWidget "/Game/Blueprints/UI/W_OverspaceHUD.W_OverspaceHUD_C" _asbp_overspace_controller self))
    (CallFunction|SetHUD _returnvalue)
    (UserInterface|Viewport|AddtoPlayerScreen (CallFunction|GetHUD))
    (else
      (Default|RegisterPlayer (CallFunction|GetGameMode) self)
      (AI|RunBehaviorTree (AI|GetAIController self) "/Game/Blueprints/AI/BT/BT_OverspaceNPC.BT_OverspaceNPC")
      (if (Variables|Default|GetroamNearSpawn)
        (Variables|Default|SetspawnLocation (Transformation|GetActorLocation))))))

(event Collision|EventActorBeginOverlap
  (params (OtherActor :type Actor%20Object%20Reference))
  (|CallParentFunction OtherActor))

(event EventTick
  (params (DeltaSeconds :type Float%20%28single-precision%29))
  (bind _returnvalue (Transformation|GetActorLocation))
  (bind _movelocation (CallFunction|GetMoveLocation))
  (bind _returnvalue_2 (Math|Rotator|FindLookatRotation _returnvalue _movelocation))
  (|CallParentFunction DeltaSeconds)
  (if (CallFunction|GetIsHumanPlayer)
    (CallFunction|SetMovementEffects)
    (elif (Variables|Default|GetmovementEnabled)
      (if (Variables|Default|GetmovingToLocation)
        (Pawn|Input|AddMovementInput (Math|Vector|GetForwardVector _returnvalue_2) 0.75 false)
        (Transformation|SetRelativeRotation (Variables|Default|GetDirection) _returnvalue_2 false false)))))

(event EventFireEventfromMessage
  (params (eventWithArguments :type String))
  (CallFunction|FireEvent eventWithArguments))

(fn ConstructionScript
  (|CallParentFunction))

(fn SpawnPlayerShips
  (if (CallFunction|GetIsHumanPlayer)
    (bind _outrownames (DataTable|GetDataTableRowNames "/Game/Blueprints/DataTables/DT_PlayerShips.DT_PlayerShips"))
    (for (_array_element _array_index) _outrownames
      (bind _returnvalue (Utilities|GetDataTableRow "/Game/Blueprints/DataTables/DT_PlayerShips.DT_PlayerShips" _array_element)
        (:then
          (CallFunction|SpawnShipinFormation _returnvalue _array_index))))
    (else
      (bind _outrownames_2 (DataTable|GetDataTableRowNames "/Game/Blueprints/DataTables/DT_NPCFleets.DT_NPCFleets"))
      (bind _array_element_2 (Utilities|Array|ForEachLoopwithBreak _outrownames_2 :!label _label)
        (:LoopBody
          (if (Utilities|String|Contains (Utilities|String|ToString(Name) _array_element_2) (Utilities|String|ToString(Text) (CallFunction|GetPlayerName)))
            (bind _returnvalue_2 (Utilities|GetDataTableRow "/Game/Blueprints/DataTables/DT_NPCFleets.DT_NPCFleets" _array_element_2)
              (:then
                (Utilities|Array|Add (LocalVariables|GetnpcShips) _returnvalue_2)))
            (elif (> (Utilities|Array|Length (LocalVariables|GetnpcShips)) 0) ; Assuming NPC ships are found in NPC groups
              (goto _label Break)
              (else
                (Development|PrintString (Utilities|String|Append "***CONSIDER REFACTORING DT_NPCFLEETS TO HAVE ARRAYS OF NPC SHIPS BY NPC NAME TO CREATE GROUPS OF SHIPS IN SINGLE DT ROW***" "") true true "(R=1.000000,G=0.500000,B=0.000000,A=1.000000)")))))
        (:Completed
          (if (> (Utilities|Array|Length (LocalVariables|GetnpcShips)) 0)
            (for (_array_element_3 _array_index_2) (LocalVariables|GetnpcShips)
              (bind _returnvalue_3 (Utilities|GetDataTableRow "/Game/Blueprints/DataTables/DT_BaseShips.DT_BaseShips" (Utilities|String|StringToName (Utilities|String|ToString(Text) (Utilities|Struct|BreakS_NPCShip _array_element_3))))
                (:then
                  (CallFunction|SpawnShipinFormation _returnvalue_3 _array_index_2))))
            (else
              (Development|PrintString (Utilities|String|Append "***UNABLE TO FIND ANY NPC SHIPS FOR " (Utilities|String|ToString(Text) (CallFunction|GetPlayerName)) " IN DT_NPCFLEETS***") true true "(R=0.500000,G=0.000000,B=0.000000,A=1.000000)"))))))))

(fn GetFormationComponentbyIndex
  (params (index :type Integer))
  (switch int index
    (:Default
      _)
    (:0
      _)
    (:1
      (return (Variables|Default|GetShipFormation2)))
    (:2
      (return (Variables|Default|GetShipFormation3)))
    (:3
      (return (Variables|Default|GetShipFormation4)))
    (:4
      (return (Variables|Default|GetShipFormation5)))
    (:5
      (return (Variables|Default|GetShipFormation6))))
  (return (Variables|Default|GetShipFormation1)))

(fn SpawnShipinFormation
  (params (shipStats :type S%20Ship%20Structure) (formationIndex :type Integer))
  (bind _shipstatuseffects (Utilities|Struct|BreakS_Ship shipStats))
  (bind _returnvalue (Game|SpawnActorfromClass "/Game/Pawns/BP_OverspaceShip.BP_OverspaceShip_C" (Transformation|GetWorldTransform (CallFunction|GetFormationComponentbyIndex formationIndex)) "AlwaysSpawn" 0 shipStats true self 0))
  (bind _output_get (LocalVariables|SetcurrentShip _returnvalue))
  (Transformation|AttachComponentToComponent _output_get (CallFunction|GetFormationComponentbyIndex formationIndex) "None" "KeepWorld" "KeepWorld" "KeepWorld" true)
  (if (> (Utilities|Array|Length _shipstatuseffects) 0)
    (for _array_element _shipstatuseffects
      (Default|AddStatusEffect (LocalVariables|GetcurrentShip) _array_element)))
  (Default|UpdateShipComponents (LocalVariables|GetcurrentShip) true))

(fn GetRandomLocationinRange
  (params (range :type Float%20%28single-precision%29))
  (LocalVariables|SetroamingRange range)
  (LocalVariables|SetrandomLocationX (Math|Random|RandomFloatinRange (* (LocalVariables|GetroamingRange) -1.0) (LocalVariables|GetroamingRange)))
  (LocalVariables|SetrandomLocationY (Math|Random|RandomFloatinRange (* (LocalVariables|GetroamingRange) -1.0) (LocalVariables|GetroamingRange)))
  (Variables|Default|SetmoveLocation (+ (select (Variables|Default|GetroamNearSpawn) (Variables|Default|GetspawnLocation) (Transformation|GetActorLocation)) (Math|Vector|MakeVector (LocalVariables|GetrandomLocationX) (LocalVariables|GetrandomLocationY) 0.0))))

(fn GetMoveLocation
  (Utilities|IsValid (Variables|Default|GetmoveToTarget)
    (:Is%20Valid
      (return (Transformation|GetActorLocation (Variables|Default|GetmoveToTarget))))
    (:Is%20Not%20Valid
      (return (Variables|Default|GetmoveLocation)))))

(fn MovetoLocation
  (params (moveToLocation :type Boolean))
  (Variables|Default|SetmovingToLocation moveToLocation))

(fn SetMovetoTarget
  (params (target :type Actor%20Object%20Reference))
  (Variables|Default|SetmoveToTarget target))

(fn SetMovementEffects
  (bind _returnvalue (Transformation|GetVelocity))
  (bind _maxflyspeed (CallFunction|GetMaxFlySpeed))
  (bind _maxflyspeed_2 (CallFunction|GetMaxFlySpeed))
  (bind _returnvalue_2 (Transformation|GetVelocity))
  (bind _charactermovement (Variables|Character|GetCharacterMovement))
  (bind _maxflightlag (Variables|Default|GetmaxFlightLag))
  (bind _maxflightlag_2 (Variables|Default|GetmaxFlightLag))
  (bind _springarm (Variables|Default|GetSpringArm))
  (bind (_x _y) (Math|Vector|BreakVector _returnvalue))
  (bind (_x_2 _y_2) (Math|Vector|BreakVector _returnvalue_2))
  (bind _maxflyspeed_3 (Variables|/Script/Engine.CharacterMovementComponent|GetMaxFlySpeed _charactermovement))
  (bind _returnvalue_3 (* _maxflyspeed_3 -1.0))
  (Transformation|SetRelativeLocation (Variables|Default|GetDirection) (Math|Vector|MakeVector (Math|Float|MapRangeClamped _x _returnvalue_3 _maxflyspeed_3 _maxflightlag (* _maxflightlag -1.0)) (Math|Float|MapRangeClamped _y _returnvalue_3 _maxflyspeed_3 _maxflightlag_2 (* _maxflightlag_2 -1.0)) 0.0) false false)
  (LocalVariables|SetcurrentSpeed (Math|Float|Clamp(Float) (+ (Math|Float|Absolute(Float) _x_2) (Math|Float|Absolute(Float) _y_2)) 0.0 (CallFunction|GetMaxFlySpeed)))
  (Variables|/Script/Engine.SpringArmComponent|SetTargetArmLength _springarm (Math|Float|MapRangeClamped (LocalVariables|GetcurrentSpeed) (* _maxflyspeed 0.2) (* _maxflyspeed 0.8) (Variables|Default|GetfullStopCameraZoom) (Variables|Default|GetfullSpeedCameraZoom)))
  (Transformation|SetRelativeRotation _springarm (Math|Rotator|MakeRotator 0.0 (Math|Float|MapRangeClamped (LocalVariables|GetcurrentSpeed) (* _maxflyspeed_2 0.2) (* _maxflyspeed_2 0.8) (Variables|Default|GetfullStopCameraPitch) (Variables|Default|GetfullSpeedCameraPitch)) 0.0) false false))

(fn GetMaxFlySpeed
  (return (Variables|/Script/Engine.CharacterMovementComponent|GetMaxFlySpeed (Variables|Character|GetCharacterMovement))))

(fn EngageTarget
  (params (player :type Actor%20Object%20Reference))
  (bind _asbp_overspace_player (Utilities|Casting|CastToBP_OverspacePlayer player)
    (:then
      (LocalVariables|SettargetPlayer _asbp_overspace_player)
      (Development|PrintString (Utilities|String|Append (Utilities|String|ToString(Text) (CallFunction|GetPlayerName)) " is engaging " (Utilities|String|ToString(Text) (Default|GetPlayerName _asbp_overspace_player))) true true "(R=1.000000,G=0.750000,B=0.000000,A=1.000000)" 5.0)
      (Variables|Default|SetmovingToLocation false)
      (CallFunction|StopAllShips)
      (Default|AssignPlayerAvatar (CallFunction|GetGameMode) self false)
      (CallFunction|AddMessagetoQueue (Utilities|Struct|MakeS_Message "I have you now!" "" "" "" "" "" "" "" "" 0.0 "" "" (Utilities|String|ToString(Text) (CallFunction|GetPlayerName)) true) false)
      (CallFunction|AddMessagetoQueue (Utilities|Struct|MakeS_Message "" "" "" "" "" "" "" "" "" 0.0 (Utilities|String|Append "StartBattle_" (Utilities|String|ToString(Text) (Default|GetPlayerName (LocalVariables|GettargetPlayer))) "_" (Utilities|String|ToString(Text) (CallFunction|GetPlayerName))) (Utilities|String|ToString(Text) (Default|GetPlayerName (LocalVariables|GettargetPlayer))) (Utilities|String|ToString(Text) (CallFunction|GetPlayerName)) true true) true))
    (:CastFailed
      (Development|PrintString (Utilities|String|Append "***UNABLE TO CAST " (Utilities|GetDisplayName player) " TO BP_OVERSPACEPLAYER***") true true "(R=0.500000,G=0.000000,B=0.004000,A=1.000000)"))))

(fn StopMovement
  (Variables|Default|SetmovementEnabled false)
  (Components|Movement|StopMovementImmediately (Variables|Character|GetCharacterMovement))
  (if (CallFunction|GetIsHumanPlayer)
    (bind _asbp_overspace_controller (Utilities|Casting|CastToBP_OverspaceController (Pawn|GetController)))
    (Default|ToggleMovement _asbp_overspace_controller false)))

(fn FireEvent
  (params (eventWithArguments :type String))
  (bind _output_get (LocalVariables|SeteventArguments (Utilities|String|ParseIntoArray eventWithArguments "_")))
  (if (Utilities|Array|IsValidIndex _output_get)
    (switch string (Utilities|Array|Get(acopy) _output_get)
      (:Default
        (Development|PrintString (Utilities|String|Append "***UNABLE TO FIND ASSOCIATED EVENT FROM MESSAGE FOR " (Utilities|Array|Get(acopy) _output_get) "***") true true "(R=0.500000,G=0.000000,B=0.000000,A=1.000000)" 5.0))
      (:StartBattle
        (|StartBattlewithArguments))
      (:Dock
        (|DockwithArguments))
      (:StopAllShips
        (CallFunction|StopAllShips))
      (:ExitDialogue
        (CallFunction|ExitDialogue false)))
    (else
      (Development|PrintString "***UNABLE TO SPLIT ARGUMENTS STRING FOR EVENT FROM MESSAGE***" true true "(R=0.500000,G=0.000000,B=0.000000,A=1.000000)" 5.0))))

(fn StopAllShips
  (bind _outactors (Actor|GetAllActorsOfClass "BP_OverspacePlayer_C"))
  (for _array_element _outactors
    (CallFunction|StopMovement _array_element)))

(fn EnableAllShipsMovement
  (bind _outactors (Actor|GetAllActorsOfClass "BP_OverspacePlayer_C"))
  (for _array_element _outactors
    (CallFunction|EnableMovement _array_element)))

(fn EnableMovement
  (Variables|Default|SetmovementEnabled true)
  (if (CallFunction|GetIsHumanPlayer)
    (bind _asbp_overspace_controller (Utilities|Casting|CastToBP_OverspaceController (Pawn|GetController)))
    (Default|ToggleMovement _asbp_overspace_controller true)))
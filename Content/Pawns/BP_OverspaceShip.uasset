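; Overspace ship pawn that builds its visuals from ShipStats, exposes those stats and switches between five socket-placed cameras.
; On BeginPlay it sets the mesh and adds engine-socket thrusters, plus faction-material shields and looping randomized idle drift when idle movement is enabled.
; A timeline drives starfield and thrust particles, with shake and sound, for warp approaches.
; Status effects toggle thruster output and socket-matched engine or weapon damage sparks.
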(event Custom|ApproachLocation
  (params (approachVector :type Vector) (offset :type Vector))
  ;[1 1 0.2] Ship Movement
  (Camera|PlayWorldCameraShake "/Game/Blueprints/Effects/ShipBoostShake.ShipBoostShake_C" "0, 0, 0" 0.0 5e+03)
  (Utilities|FlowControl|Sequence
    (:then_0
      (bind (_direction _movementalpha _starsize _starburst _thrust) (Timeline|ApproachVectorToTarget PlayFromStart)
        (:Update
          (|SetParticleParams _starsize _starburst _thrust))
        (:RefreshStarfield
          (Components|Activation|Activate (Variables|Default|GetStarfield) true))))
    (:then_1
      (Audio|SpawnSoundAttached "/Game/SFX/Cues/Wav_WarpEngine7_End_Cue.Wav_WarpEngine7_End_Cue" (Variables|Default|GetShipBody) "None" "0, 0, 0" "0, 0, 0" "SnapToTargetIncludingScale" false 1.0 1.0 0.0 "/Game/SFX/Attenuation/EngineAttenuation.EngineAttenuation" "/Game/SFX/Concurrency/EngineConcurrency.EngineConcurrency"))))

(event Custom|RemoveShip
  ;[0.2705 0.6038 0.7758] Spawning and Removing
  (CallFunction|RemoveAllComponents)
  (Actor|DestroyActor))

(event Custom|IdleFlightMovement
  ;[1 1 0.2] Ship Movement
  (|IdleFlightMovement))

(event Custom|UpdateShipComponents
  (params (componentDamaged :type Boolean))
  (bind _returnvalue (Math|Float|SelectFloat 0.0 1.0 componentDamaged))
  (bind _weaponsparks (Variables|ShipComponents|GetweaponSparks))
  (bind _enginesparks (Variables|ShipComponents|GetengineSparks))
  ;[1 1 1] Update Ship Components
  (if (Utilities|Array|ContainsItem (Variables|ShipStats|GetstatusEffects) "NewEnumerator0")
    (for _array_element (Variables|ShipComponents|GetThrusters)
      (Effects|Components|ParticleSystem|SetFloatParameter _array_element "ThrustSpawn" _returnvalue)
      (Effects|Components|ParticleSystem|SetFloatParameter _array_element "BoostSpawn" _returnvalue))
    (if componentDamaged
      (ShipComponents|SpawnComponentDamageParticles _enginesparks "EnginePoint")
      (else
        (ShipComponents|RemoveComponentDamageParticles _enginesparks)))
    (elif (Utilities|Array|ContainsItem (Variables|ShipStats|GetstatusEffects) "NewEnumerator1")
      (if componentDamaged
        (ShipComponents|SpawnComponentDamageParticles _weaponsparks "WeaponPoint")
        (else
          (ShipComponents|RemoveComponentDamageParticles _weaponsparks))))))

(event Custom|RemoveAllComponents
  ;[0.2705 0.6038 0.7758] Spawning and Removing
  (Actor|DestroyActor (Variables|ShipComponents|Getshields))
  (ShipComponents|RemoveComponentDamageParticles (Variables|ShipComponents|GetweaponSparks))
  (ShipComponents|RemoveComponentDamageParticles (Variables|ShipComponents|GetengineSparks)))

(event EventBeginPlay
  ;[0.2705 0.6038 0.7758] Spawning and Removing
  (Components|StaticMesh|SetStaticMesh (Variables|Default|GetShipBody) (Utilities|Struct|BreakS_Ship (Variables|ShipStats|GetshipStats)))
  (|AttachShipComponents)
  (ShipSockets|SetCameraSocketLocations)
  (if (Variables|ShipMovement|GetenableIdleMovement)
    (CallFunction|IdleFlightMovement)
    (else
      (Components|Activation|Deactivate (Variables|Default|GetStarfield)))))

(fn ConstructionScript)

(fn GetShipName
  (return (Utilities|Struct|BreakS_Ship (Variables|ShipStats|GetshipStats))))

(fn GetShipType
  (return (Utilities|Struct|BreakS_Ship (Variables|ShipStats|GetshipStats))))

(fn GetAttacks
  (return (Utilities|Struct|BreakS_Ship (Variables|ShipStats|GetshipStats))))

(fn GetShipHealth
  (bind _shipstats (Variables|ShipStats|GetshipStats))
  (bind (_shiphull _totalshiphull _shipshield _totalshipshield) (Utilities|Struct|BreakS_Ship _shipstats))
  (return _shiphull _totalshiphull _shipshield _totalshipshield))

(fn GetStatusEffects
  (return (Variables|ShipStats|GetstatusEffects)))

(fn GetIsinFleet
  (return (Utilities|Struct|BreakS_Ship (Variables|ShipStats|GetshipStats))))

(fn GetShipStats
  (return (Variables|ShipStats|GetshipStats)))

(fn GetHasFleetAdmiral
  (return (Utilities|Struct|BreakS_Ship (Variables|ShipStats|GetshipStats))))

(fn SwitchCamera
  (params (camIndex :type Integer))
  (bind _debugmessages (Variables|Default|GetdebugMessages))
  (bind _debugmessages_2 (Variables|Default|GetdebugMessages))
  (bind _debugmessages_3 (Variables|Default|GetdebugMessages))
  (bind _debugmessages_4 (Variables|Default|GetdebugMessages))
  (bind _debugmessages_5 (Variables|Default|GetdebugMessages))
  (switch int camIndex
    (:1
      (ShipCameras|SetActiveCamera (Variables|Default|GetAngledCam) (Variables|Default|GetAngledSpringArm))
      (Development|PrintString "Switch to Angled Cam" _debugmessages _debugmessages "(R=0.000000,G=0.184475,B=0.467784,A=1.000000)"))
    (:2
      (ShipCameras|SetActiveCamera (Variables|Default|GetFrontCam) (Variables|Default|GetFrontSpringArm))
      (Development|PrintString "Switch to Front Cam" _debugmessages_3 _debugmessages_3 "(R=0.000000,G=0.184475,B=0.467784,A=1.000000)"))
    (:3
      (ShipCameras|SetActiveCamera (Variables|Default|GetBackCam) (Variables|Default|GetBackSpringArm))
      (Development|PrintString "Switch to Back Cam" _debugmessages_5 _debugmessages_5 "(R=0.000000,G=0.184475,B=0.467784,A=1.000000)"))
    (:4
      (ShipCameras|SetActiveCamera (Variables|Default|GetWeaponCam) (Variables|Default|GetWeaponSpringArm))
      (Development|PrintString "Switch to Weapon Cam" _debugmessages_2 _debugmessages_2 "(R=0.000000,G=0.184475,B=0.467784,A=1.000000)"))
    (:5
      (ShipCameras|SetActiveCamera (Variables|Default|GetHangarCamera) (Variables|Default|GetHangarSpringArm))
      (Development|PrintString "Switch to Weapon Cam" _debugmessages_4 _debugmessages_4 "(R=0.000000,G=0.184475,B=0.467784,A=1.000000)"))))

(fn SetActiveCamera
  (params (camera :type Camera%20Component%20Object%20Reference) (springArm :type Spring%20Arm%20Component%20Object%20Reference))
  (if (!= (Variables|Default|GetactiveCam) 0)
    (Components|Activation|SetActive (Variables|Default|GetactiveCam) false false))
  (Components|Activation|SetActive camera true false)
  (Variables|Default|SetactiveCam camera)
  (Variables|Default|SetactiveSpringArm springArm))

(fn SetCameraSocketLocations
  (Transformation|SetWorldTransform (Variables|Default|GetWeaponSpringArm) (Transformation|GetSocketTransform (Variables|Default|GetShipBody) "WeaponCam" "RTS_World") false false)
  (Transformation|SetWorldTransform (Variables|Default|GetAngledSpringArm) (Transformation|GetSocketTransform (Variables|Default|GetShipBody) "AngleCam" "RTS_World") false false)
  (Transformation|SetWorldTransform (Variables|Default|GetFrontSpringArm) (Transformation|GetSocketTransform (Variables|Default|GetShipBody) "FrontCam" "RTS_World") false false)
  (Transformation|SetWorldTransform (Variables|Default|GetBackSpringArm) (Transformation|GetSocketTransform (Variables|Default|GetShipBody) "BackCam" "RTS_World") false false)
  (Transformation|SetWorldTransform (Variables|Default|GetHangarSpringArm) (Transformation|GetSocketTransform (Variables|Default|GetShipBody) "HangarCam" "RTS_World") false false))

(fn SpawnParticleEffectatSocket
  (params (particleEffect :type Particle%20System%20Object%20Reference) (socketName :type Name))
  (Effects|SpawnEmitterAttached particleEffect (Variables|Default|GetShipBody) socketName "0, 0, 0" "0, 0, 0" "1.000000,1.000000,1.000000" "SnapToTarget"))

(fn GetAttackPoint
  (return (Transformation|GetSocketLocation (Variables|Default|GetShipBody) "AttackPoint")))

(fn ToggleShipDamage
  (params (enableDamageVFX :type Boolean) (critical :type Boolean))
  (if enableDamageVFX
    (if critical
      (Components|Activation|Activate (Variables|Default|GetSparks) false)
      (Components|Activation|Activate (Variables|Default|GetSmoke) false)
      (else
        (Components|Activation|Activate (Variables|Default|GetSparks) false)
        (Components|Activation|Deactivate (Variables|Default|GetSmoke))))
    (else
      (Components|Activation|Deactivate (Variables|Default|GetSparks))
      (Components|Activation|Deactivate (Variables|Default|GetSmoke)))))

(fn GetIsCriticallyDamaged
  (return (Utilities|Struct|BreakS_Ship (Variables|ShipStats|GetshipStats))))

(fn GetSocketTransform
  (params (socket :type Name))
  (return (Transformation|GetSocketTransform (Variables|Default|GetShipBody) socket "RTS_World")))

(fn SpawnComponentDamageParticles
  (params (componentDamageArray :type Array%20of%20Particle%20System%20Component%20Object%20References) (socketType :type String))
  (for _array_element (Transformation|GetAllSocketNames (Variables|Default|GetShipBody))
    (if (Utilities|String|Contains (Utilities|String|ToString(Name) _array_element) socketType)
      (bind _returnvalue (Effects|SpawnEmitterAttached "/Game/Realistic_Starter_VFX_Pack_Vol2/Particles/Sparks/P_Sparks_Dmg.P_Sparks_Dmg" (Variables|Default|GetShipBody) _array_element (* (Math|Vector|GetForwardVector (.rotation (Transformation|GetSocketTransform (Variables|Default|GetShipBody) _array_element "RTS_World"))) 8) "0, 0, 0" "0.500000,0.500000,0.500000" "SnapToTarget"))
      (Utilities|Array|Add componentDamageArray _returnvalue))))

(fn RemoveComponentDamageParticles
  (params (componentDamageArray :type Array%20of%20Particle%20System%20Component%20Object%20References))
  (for _array_element componentDamageArray
    (Components|DestroyComponent _array_element))
  (Utilities|Array|Clear componentDamageArray))

(fn SetThrusterBoost
  (params (boostAlpha :type Float%20%28single-precision%29))
  (for _array_element (Variables|ShipComponents|GetThrusters)
    (Effects|Components|ParticleSystem|SetVectorParameter _array_element "ThrustSize" (Math|Vector|MakeVector boostAlpha boostAlpha boostAlpha))
    (Effects|Components|ParticleSystem|SetVectorParameter _array_element "BoostSize" (Math|Vector|MakeVector boostAlpha boostAlpha boostAlpha))))

(fn GetShipOfficersNames
  (return (Utilities|Struct|BreakS_Ship (Variables|ShipStats|GetshipStats))))

(fn GetShipLevel
  (return (Math|Float|Truncate (Utilities|Struct|BreakS_Ship (Variables|ShipStats|GetshipStats)))))

(fn GetShipMesh
  (return (Variables|/Script/Engine.StaticMeshComponent|GetStaticMesh (Variables|Default|GetShipBody))))

(fn AddStatusEffect
  (params (newStatusEffect :type E_StatusTypes%20Enum%20%28by%20ref%29 :default "NewEnumerator0"))
  (Utilities|Array|AddUnique (Variables|ShipStats|GetstatusEffects) newStatusEffect)
  (CallFunction|UpdateShipComponents true))
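; BP_ScannerObject renders a hologram preview of a scanned player fleet ship, planet or dock base to a render target.
; A SceneCapture2D shows only this actor, while SetScannerObject casts the target to pick mesh, scale and hologram material.
; Four widgets snap to mesh sockets, showing ship attacks or hardcoded planet points of interest.
; SetPlanetMenuScan instead shows a plain sphere, hides the stats and moves the spring arm to a socket.
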(event EventBeginPlay
  (Utilities|Array|Add (Variables|/Script/Engine.SceneCaptureComponent|GetShowOnlyActors (Variables|Default|GetSceneCaptureComponent2D)) self)
  (Utilities|Array|Add (Variables|Default|GetscannerStatWigets) (Variables|Default|GetScannerStat1))
  (Utilities|Array|Add (Variables|Default|GetscannerStatWigets) (Variables|Default|GetScannerStat2))
  (Utilities|Array|Add (Variables|Default|GetscannerStatWigets) (Variables|Default|GetScannerStat3))
  (Utilities|Array|Add (Variables|Default|GetscannerStatWigets) (Variables|Default|GetScannerStat4)))

(fn ConstructionScript)

(fn GetSceneCaptureTexture
  (return (Variables|/Script/Engine.SceneCaptureComponent2D|GetTextureTarget (Variables|Default|GetSceneCaptureComponent2D))))

(fn SetSceneCaptureTexture
  (params (TextureTarget :type Texture%20Render%20Target%202D%20Object%20Reference))
  (Variables|/Script/Engine.SceneCaptureComponent2D|SetTextureTarget (Variables|Default|GetSceneCaptureComponent2D) TextureTarget))

(fn SetScannerObject
  (params (scannerObject :type Actor%20Object%20Reference))
  (bind _asbp_overspace_player (Utilities|Casting|CastToBP_OverspacePlayer scannerObject)
    (:then
      (Components|StaticMesh|SetStaticMesh (Variables|Default|GetScannerObject) (Default|GetShipMesh (Utilities|Array|Get(acopy) (Default|GetFleetShips _asbp_overspace_player))))
      (CallFunction|SetMeshScale 1.0)
      (CallFunction|SetMeshMaterials "/Game/Materials/Outline/MI_ScannerSchemaHologram.MI_ScannerSchemaHologram")
      (CallFunction|SetShipScannerStats (Default|GetAttacks (Utilities|Array|Get(acopy) (Default|GetFleetShips _asbp_overspace_player)))))
    (:CastFailed
      (bind _asbp_dockable_planet (Utilities|Casting|CastToBP_DockablePlanet scannerObject)
        (:then
          (Components|StaticMesh|SetStaticMesh (Variables|Default|GetScannerObject) (Default|GetBaseMesh _asbp_dockable_planet))
          (CallFunction|SetMeshScale 25.0)
          (CallFunction|SetMeshMaterials "/Game/Materials/Outline/MI_ScannerSchemaHologram.MI_ScannerSchemaHologram")
          (CallFunction|SetPlanetScannerStats (Utilities|Array|MakeArray "Ancient Ruins" "Gimbal Base" "Distress Beacon" "Periapsis Space Port")))
        (:CastFailed
          (bind _asbp_dock_base (Utilities|Casting|CastToBP_DockBase scannerObject)
            (:then
              (Components|StaticMesh|SetStaticMesh (Variables|Default|GetScannerObject) (Default|GetBaseMesh _asbp_dock_base))
              (CallFunction|SetMeshScale 1.0)
              (CallFunction|SetMeshMaterials "/Game/Materials/Outline/MI_ScannerBaseHologram.MI_ScannerBaseHologram"))
            (:CastFailed
              (Development|PrintString (Utilities|String|Append "***UNABLE TO SET SCANNER MESH FOR " (Utilities|GetDisplayName scannerObject) "***")))))))))

(fn SetShipScannerStats
  (params (attacks :type Array%20of%20Texts))
  (for (_array_element _array_index) (Variables|Default|GetshipStatSockets)
    (if (Utilities|Array|IsValidIndex attacks _array_index)
      (Transformation|SetRelativeLocation (Utilities|Array|Get(acopy) (Variables|Default|GetscannerStatWigets) _array_index) (- (Transformation|GetSocketLocation (Variables|Default|GetScannerObject) _array_element) (Transformation|GetActorLocation)) false false)
      (Default|SetQuickStat (.AsW%20HUDScanner%20Stat (Utilities|Casting|CastToW_HUDScannerStat (UserInterface|GetUserWidgetObject (Utilities|Array|Get(acopy) (Variables|Default|GetscannerStatWigets) _array_index)))) (Utilities|String|ToString(Text) (Utilities|Array|Get(acopy) attacks _array_index)) (not (or (Utilities|Name|Equal(Name) _array_element "WeaponPoint1") (Utilities|Name|Equal(Name) _array_element "DockingPoint"))))
      (Default|ToggleScannerStat (.AsW%20HUDScanner%20Stat (Utilities|Casting|CastToW_HUDScannerStat (UserInterface|GetUserWidgetObject (Utilities|Array|Get(acopy) (Variables|Default|GetscannerStatWigets) _array_index)))) true))))

(fn SetMeshScale
  (params (scale :type Float%20%28single-precision%29))
  (Transformation|SetRelativeScale3D (Variables|Default|GetScannerObject) (Math|Vector|MakeVector scale scale scale)))

(fn SetMeshMaterials
  (params (meshMaterial :type Material%20Interface%20Object%20Reference))
  (for _array_element (Class|MeshComponent|GetMaterialSlotNames (Variables|Default|GetScannerObject))
    (Rendering|Material|SetMaterialbyName (Variables|Default|GetScannerObject) _array_element meshMaterial)))

(fn SetPlanetScannerStats
  (params (pointsOfInterest :type Array%20of%20Texts))
  (for (_array_element _array_index) (Variables|Default|GetplanetStatSockets)
    (if (Utilities|Array|IsValidIndex pointsOfInterest _array_index)
      (Transformation|SetRelativeLocation (Utilities|Array|Get(acopy) (Variables|Default|GetscannerStatWigets) _array_index) (- (Transformation|GetSocketLocation (Variables|Default|GetScannerObject) _array_element) (Transformation|GetActorLocation)) false false)
      (Default|SetQuickStat (.AsW%20HUDScanner%20Stat (Utilities|Casting|CastToW_HUDScannerStat (UserInterface|GetUserWidgetObject (Utilities|Array|Get(acopy) (Variables|Default|GetscannerStatWigets) _array_index)))) (Utilities|String|ToString(Text) (Utilities|Array|Get(acopy) pointsOfInterest _array_index)) (Math|Random|RandomBool))
      (Default|ToggleScannerStat (.AsW%20HUDScanner%20Stat (Utilities|Casting|CastToW_HUDScannerStat (UserInterface|GetUserWidgetObject (Utilities|Array|Get(acopy) (Variables|Default|GetscannerStatWigets) _array_index)))) true))))

(fn SetPlanetMenuScan
  (Components|StaticMesh|SetStaticMesh (Variables|Default|GetScannerObject) "/Game/Models/SM_Sphere.SM_Sphere")
  (CallFunction|SetMeshScale 25.0)
  (CallFunction|SetMeshMaterials "/Game/Materials/Outline/MI_ScannerSchemaHologram.MI_ScannerSchemaHologram")
  (for _array_element (Variables|Default|GetscannerStatWigets)
    (Default|ToggleScannerStat (.AsW%20HUDScanner%20Stat (Utilities|Casting|CastToW_HUDScannerStat (UserInterface|GetUserWidgetObject _array_element))) false))
  (Transformation|SetWorldLocation (Variables|Default|GetSpringArm) (Transformation|GetSocketLocation (Variables|Default|GetScannerObject) (Utilities|Array|Get(acopy) (Variables|Default|GetplanetStatSockets))) false false))